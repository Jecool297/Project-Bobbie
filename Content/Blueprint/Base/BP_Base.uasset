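; Mission base for the player's boat that starts a castaway rescue and checks for victory.
; Entering the launch zone before the mission starts spawns two castaways at arrow positions, refills boat health and plays a flare cutscene with input disabled and damping raised.
; The end zone compares rescued and required counts, then plays the final sequence and victory message or prints that people are missing.
; Array-based castaway placement is unfinished and never runs.
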(event `self.ReceiveBeginPlay`
  (bind _asbp_boat_template (cast `/Game/Blueprint/Bateaux/Bobbie/BP_BoatTemplate` (`GameplayStatics.GetPlayerPawn` 0)))
  (set `self.Bobbie_Ref` _asbp_boat_template))

(event `self.ReceiveTick`
  (params (DeltaSeconds :type "Float (single-precision)")))

(event `self.ZoneLancementMission.OnComponentBeginOverlap`
  (params (OverlappedComponent :type "PrimitiveComponent Object Reference") (OtherActor :type "Actor Object Reference") (OtherComp :type "PrimitiveComponent Object Reference") (OtherBodyIndex :type Integer) (bFromSweep :type Boolean) (SweepResult :type "HitResult Structure (by ref)"))
  (bind _bobbie_ref (`self.Bobbie_Ref`))
  (if (and (== OtherActor (`GameplayStatics.GetPlayerPawn` 0)) (not (`self.MissionLance?`)))
    ;[1 1 1] Lance l'apparition des naufragés dans le niveau
    (`self.AppartitionDesNaufrages`)
    (set `/Game/Blueprint/Bateaux/Bobbie/BP_BoatTemplate.SanteBobbie` 100.0 _bobbie_ref)
    (`/Game/Widget/WBP_UI_Jeu.MiseAJourVie` (`/Game/Blueprint/Bateaux/Bobbie/BP_BoatTemplate.UI_EnJeu` _bobbie_ref))))

(event `self.ZoneFinMission.OnComponentBeginOverlap`
  (params (OverlappedComponent :type "PrimitiveComponent Object Reference") (OtherActor :type "Actor Object Reference") (OtherComp :type "PrimitiveComponent Object Reference") (OtherBodyIndex :type Integer) (bFromSweep :type Boolean) (SweepResult :type "HitResult Structure (by ref)"))
  (if (== OtherActor (`GameplayStatics.GetPlayerPawn` 0))
    ;[1 1 1] Vérifie si le nombre de naufragés actuellement récupéré correspond au nombre de naufragés à sauver dans le niveau.
    (if (== (`self.PersonnesRequises`) (`/Game/Blueprint/Bateaux/Bobbie/BP_BoatTemplate.IndexPersonneSecouru` (`self.Bobbie_Ref`)))
      ;[1 1 1] Condition de victoire
      (bind (_outactor _returnvalue) (`LevelSequencePlayer.CreateLevelSequencePlayer` "/Game/Sequencer/LS_SequenceFinale.LS_SequenceFinale"))
      (add `MovieSceneSequencePlayer.OnFinished` _returnvalue (delegate `OnFinished_Event`))
      (`MovieSceneSequencePlayer.Play` _returnvalue)
      (`PrimitiveComponent.SetLinearDamping` (`/Game/Blueprint/Bateaux/Bobbie/BP_BoatTemplate.SM_Bobbie` (`self.Bobbie_Ref`)) 1.0)
      (else
        ;[1 1 1] Condition lorsqu'il manque des naufragés
        (`KismetSystemLibrary.PrintString` "Il manque des personnes")))))

(event `OnFinished_Event`
  ;[1 1 1] Condition de victoire
  (`/Game/Widget/WBP_UI_Jeu.MessageFinVictoire` (`/Game/Blueprint/Bateaux/Bobbie/BP_BoatTemplate.UI_EnJeu` (`self.Bobbie_Ref`)) "Visible"))

(event `AppartitionDesNaufrages`
  ;[1 1 1] Fait apparaitre les naufragés à leurs endroit respectif (Position des ''Arrows'' du BP_Base)
  (`self.CinematiqueDeCamera`)
  (set `self.MissionLance?` true)
  (bind _returnvalue (`|SpawnActorFromClass` "/Game/Blueprint/Naufrages/BP_NaufrageV2.BP_NaufrageV2_C" (`KismetMathLibrary.MakeTransform` (`SceneComponent.K2_GetComponentLocation` (`self.PositionNaufragee1`))) "Undefined" "MultiplyWithRoot" null null))
  (set `self.Naufrage01` _returnvalue)
  (bind _returnvalue_2 (`|SpawnActorFromClass` "/Game/Blueprint/Naufrages/BP_NaufrageV2.BP_NaufrageV2_C" (`KismetMathLibrary.MakeTransform` (`SceneComponent.K2_GetComponentLocation` (`self.PositionNaufragee2`))) "Undefined" "MultiplyWithRoot" null null))
  (set `self.Naufrage02` _returnvalue_2))

(event `CinematiqueDeCamera`
  (bind (_outactor _returnvalue) (`LevelSequencePlayer.CreateLevelSequencePlayer` "/Game/Sequencer/LS_FeuDetresse.LS_FeuDetresse"))
  (add `MovieSceneSequencePlayer.OnFinished` _returnvalue (delegate `CinematiqueFlareFin`))
  (`MovieSceneSequencePlayer.Play` _returnvalue)
  (`PrimitiveComponent.SetLinearDamping` (`/Game/Blueprint/Bateaux/Bobbie/BP_BoatTemplate.SM_Bobbie` (`self.Bobbie_Ref`)) 5.0)
  (`self.DisableInput` (`self.Bobbie_Ref`) (`GameplayStatics.GetPlayerController` 0))
  (`KismetSystemLibrary.Delay` 3.0)
  (`/Game/Blueprint/Naufrages/BP_NaufrageV2.LancerFusee` (`self.Naufrage02`))
  (`/Game/Blueprint/Naufrages/BP_NaufrageV2.LancerFusee` (`self.Naufrage01`)))

(event `CinematiqueFlareFin`
  (bind _bobbie_ref (`self.Bobbie_Ref`))
  (`self.EnableInput` _bobbie_ref (`GameplayStatics.GetPlayerController` 0))
  (`PrimitiveComponent.SetLinearDamping` (`/Game/Blueprint/Bateaux/Bobbie/BP_BoatTemplate.SM_Bobbie` _bobbie_ref) 0.0)
  (`/Game/Widget/WBP_UI_Jeu.AffichageAideNaufrage` (`/Game/Blueprint/Bateaux/Bobbie/BP_BoatTemplate.UI_EnJeu` _bobbie_ref) "Visible"))

(fn `AjouterUnNaufrage`)

(fn `UserConstructionScript`)