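; Parent template Blueprint for navigation buoys (lateral, cardinal, isolated danger, safe water) that return to their starting spot after being hit.
; ChangerTypeDeBouees picks mesh, capsule and mass scale by family and variant; the construction script calls it with the Charpentes family.
; BeginPlay saves the initial transform.
; A hit stops any move and starts a three-second timer, then MoveComponentTo eases the mesh toward that transform, lowered in Z, printing debug status.
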(event `self.ReceiveBeginPlay`
  ;[1 1 1] Enregistrement de la position initiale
  (set `self.TransformationInitiale` (`self.GetTransform`)))

(event `self.Bouees.OnComponentHit`
  (params (HitComponent :type "PrimitiveComponent Object Reference") (OtherActor :type "Actor Object Reference") (OtherComp :type "PrimitiveComponent Object Reference") (NormalImpulse :type "Vector Structure") (Hit :type "HitResult Structure (by ref)"))
  (bind (_transformationinitiale_location _transformationinitiale_rotation) (`KismetMathLibrary.BreakTransform` (`self.TransformationInitiale`)))
  ;[1 1 1] Retour à la position initial 3 secondes après l'impacte avec tout objet.
  (`KismetSystemLibrary.K2_SetTimerDelegate` (delegate `RetourPositionInitale`) 3.0)
  (goto _label :!via `Stop`))

(event `RetourPositionInitale`
  (bind (_transformationinitiale_location _transformationinitiale_rotation) (`KismetMathLibrary.BreakTransform` (`self.TransformationInitiale`)))
  ;[1 1 1] Retour à la position initial 3 secondes après l'impacte avec tout objet.
  (`self.PrintInfos` "Mouvement Bouées:" "En cours de Déplacement " (struct :`R` 1.0 :`G` 0.958267 :`A` 1.0) 10.0)
  (`KismetSystemLibrary.MoveComponentTo` (`self.Bouees`) (+ _transformationinitiale_location (0.0 0.0 -100.0)) _transformationinitiale_rotation true true (`self.DureeDeplacement`) :!label _label)
  (`self.PrintInfos` "Mouvement Bouées:" "Arrivée au point de départ" (struct :`R` 0.114152 :`G` 1.0 :`A` 1.0) 10.0))

(fn `ChangerTypeDeBouees`
  (params (`Type de bouees` :type "/Game/Blueprint/Bouees/Enumerations/Enum_TypesBouees Enum (by ref)"))
  (locals (MassMaximum :type "Float (double-precision)" :default 2.0))
  (bind _bouees (`self.Bouees`))
  (bind _bouees_2 (`self.Bouees`))
  (bind _capsule (`self.Capsule`))
  (bind _capsule_2 (`self.Capsule`))
  (bind _capsule_3 (`self.Capsule`))
  (bind _bouees_3 (`self.Bouees`))
  (switch `/Game/Blueprint/Bouees/Enumerations/Enum_TypesBouees` `Type de bouees`
    (:`NewEnumerator0`
      ;[1 1 1] Changement emtre les bouées à charpente (Plus lourde)
      (switch `/Game/Blueprint/Bouees/Enumerations/Enum_TypesBouees_Charpente` (`self.Type de bouees Charpente`)
        (:`NewEnumerator0`
          (`StaticMeshComponent.SetStaticMesh` _bouees_3 "/Game/Art/Bouees/SM_Bouees_SM_DangerIsole_Charpente.SM_Bouees_SM_DangerIsole_Charpente")
          (`CapsuleComponent.SetCapsuleSize` _capsule_3 70.0 200.0 true))
        (:`NewEnumerator1`
          (`StaticMeshComponent.SetStaticMesh` _bouees_3 "/Game/Art/Bouees/SM_Bouees_SM_LateraleVerte_Charpente.SM_Bouees_SM_LateraleVerte_Charpente")
          (`CapsuleComponent.SetCapsuleSize` _capsule_3 55.0 160.0 true :!label _label))
        (:`NewEnumerator2`
          (`StaticMeshComponent.SetStaticMesh` _bouees_3 "/Game/Art/Bouees/SM_Bouees_SM_LateraleRouge_Charpente.SM_Bouees_SM_LateraleRouge_Charpente")
          (goto _label))
        (:`NewEnumerator3`
          (`StaticMeshComponent.SetStaticMesh` _bouees_3 "/Game/Art/Bouees/SM_Bouees_SM_Pillarbuoy_030.SM_Bouees_SM_Pillarbuoy_030")
          (goto _label)))
      (`SceneComponent.K2_AddRelativeLocation` _capsule_3 (0.0 0.0 0.0) false false)
      (`PrimitiveComponent.SetMassScale` (`self.Bouees`) "None" (`local.MassMaximum`)))
    (:`NewEnumerator1`
      ;[1 1 1] Changement entre les bouées espar (Taille Moyenne )
      (switch `/Game/Blueprint/Bouees/Enumerations/Enum_TypesBouees_Espar` (`self.Type Bouees Espar`)
        (:`NewEnumerator0`
          (`StaticMeshComponent.SetStaticMesh` _bouees_2 "/Game/Art/Bouees/SM_Bouees_SM_DangerIsole_Espar.SM_Bouees_SM_DangerIsole_Espar")
          (`CapsuleComponent.SetCapsuleSize` _capsule_2 35.0 75.0 true :!label _label_2)
          (`SceneComponent.K2_AddRelativeLocation` _capsule_2 (0.0 0.0 -150.0) false false))
        (:`NewEnumerator1`
          (`StaticMeshComponent.SetStaticMesh` _bouees_2 "/Game/Art/Bouees/SM_Bouees_SM_LateralesVerte_Espar.SM_Bouees_SM_LateralesVerte_Espar")
          (goto _label_2))
        (:`NewEnumerator2`
          (`StaticMeshComponent.SetStaticMesh` _bouees_2 "/Game/Art/Bouees/SM_Bouees_SM_LateraleRouge_Conique.SM_Bouees_SM_LateraleRouge_Conique")
          (goto _label_2))
        (:`NewEnumerator3`
          (`StaticMeshComponent.SetStaticMesh` _bouees_2 "/Game/Art/Bouees/SM_Bouees_SM_EauxSaine_Espar.SM_Bouees_SM_EauxSaine_Espar")))
      (`PrimitiveComponent.SetMassScale` (`self.Bouees`) "None" (/ (`local.MassMaximum`) 2.0)))
    (:`NewEnumerator2`
      ;[1 1 1] Changements entre les type de bouées cardinales
      (switch `/Game/Blueprint/Bouees/Enumerations/Enum_TypesBouees_Cardinales` (`self.Type de bouees Cardinales`)
        (:`NewEnumerator0`
          (`StaticMeshComponent.SetStaticMesh` _bouees "/Game/Art/Bouees/SM_Bouees_SM_Cardinales_Nord.SM_Bouees_SM_Cardinales_Nord"))
        (:`NewEnumerator1`
          (`StaticMeshComponent.SetStaticMesh` _bouees "/Game/Art/Bouees/SM_Bouees_SM_Cardinales_Sud.SM_Bouees_SM_Cardinales_Sud"))
        (:`NewEnumerator2`
          (`StaticMeshComponent.SetStaticMesh` _bouees "/Game/Art/Bouees/SM_Bouees_SM_Cardinales_Ouest.SM_Bouees_SM_Cardinales_Ouest"))
        (:`NewEnumerator3`
          (`StaticMeshComponent.SetStaticMesh` _bouees "/Game/Art/Bouees/SM_Bouees_SM_Cardinales_Est.SM_Bouees_SM_Cardinales_Est")))
      (`CapsuleComponent.SetCapsuleSize` _capsule 55.0 160.0 true)
      (`SceneComponent.K2_AddRelativeLocation` _capsule (0.0 0.0 0.0) false false)
      (`PrimitiveComponent.SetMassScale` (`self.Bouees`) "None" (`local.MassMaximum`)))))

(fn `PrintInfos`
  (params (NomDeValeur :type String) (Valeur :type String) (CouleurTexte :type "LinearColor Structure") (Duration :type "Float (single-precision)") (`Print À l'écran?` :type Boolean :default true))
  (`KismetSystemLibrary.PrintString` (`KismetStringLibrary.Concat_StrStr` NomDeValeur Valeur) `Print À l'écran?` true CouleurTexte Duration))

(fn `UserConstructionScript`
  (`self.ChangerTypeDeBouees` "NewEnumerator0"))