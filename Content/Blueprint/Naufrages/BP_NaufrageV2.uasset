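; BP_NaufrageV2 is a shipwreck survivor with a life buoy that the player's boat, Bobbie, can rescue.
; While Bobbie is inside its slowdown sphere and not aiming, Tick applies a radial force scaled by orientation, distance, speed and throttle input.
; Zone overlaps toggle Bobbie's forced look, light and rescue UI; a hit buoy glides back toward its start after a delay.
; It also spawns distress flares and increments the rescue count.
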(event `self.ReceiveTick`
  (params (DeltaSeconds :type "Float (single-precision)"))
  (bind _returnvalue (`self.K2_GetActorLocation`))
  (bind _bobbie_ref (`self.Bobbie_Ref`))
  (bind _returnvalue_2 (`self.K2_GetActorLocation` _bobbie_ref))
  (bind _returnvalue_3 (`KismetMathLibrary.Vector_Distance` _returnvalue _returnvalue_2))
  (bind _returnvalue_4 (/ (`SphereComponent.SphereRadius` (`self.ZoneDeRalentissement`)) 2.0))
  (bind _returnvalue_5 (`KismetMathLibrary.Normal` (- _returnvalue_2 _returnvalue)))
  (bind _returnvalue_6 (`KismetMathLibrary.MapRangeClamped` _returnvalue_3 _returnvalue_4 0.0 0.0 _returnvalue_4))
  (bind _returnvalue_7 (`KismetMathLibrary.Dot_VectorVector` _returnvalue_5 (`self.GetActorForwardVector` (`self.Bobbie_Ref`))))
  (if (and (`self.RalentissementBobbie?`) (not (`/Game/Blueprint/Bateaux/Bobbie/BP_BoatTemplate.ModeViseActive` (`self.Bobbie_Ref`))))
    ;[1 1 1] Regarde si la touche d'accélération est appuyé
    (set `self.AccelerationActive?` (or (> (`|GetInputActionValue`) 0.0) (> (`|GetInputActionValue`) 0.0)))
    (set `self.DerniereDistanceSurRayon` _returnvalue_3)
    (bind _retourdeforce (`self.CalculForceProportionelle` (`self.Bobbie_Ref`) _returnvalue_6))
    (`PrimitiveComponent.AddForce` (`/Game/Blueprint/Bateaux/Bobbie/BP_BoatTemplate.SM_Bobbie` _bobbie_ref) (* _returnvalue_5 (`KismetMathLibrary.SelectFloat` 0.0 (* (`KismetMathLibrary.Abs` _returnvalue_7) (`KismetMathLibrary.SelectFloat` (* _retourdeforce (`self.ForceRalentissement`)) (* (/ (`self.ForceRalentissement`) 100.0) (`KismetMathLibrary.SelectFloat` (* (`/Game/Blueprint/Bateaux/Bobbie/BP_BoatTemplate.VelociteGlobale` _bobbie_ref) _returnvalue_6) 1.0 (`self.AccelerationActive?`))) (> _returnvalue_6 (/ _returnvalue_4 2.0)))) (< _returnvalue_7 0.0))) "None" false)
    (`KismetSystemLibrary.PrintString` (`KismetStringLibrary.Concat_StrStr` "Orientation bobbie to Naufrage" (`KismetStringLibrary.Conv_DoubleToString` _returnvalue_7)))))

(event `self.ReceiveBeginPlay`
  ;[1 1 1] Enregistrement de la position initiale
  (set `self.TransformationInitiale` (`self.GetTransform`))
  ;[1 1 1] Référence à Bobbie
  (bind _asbp_boat_template (cast `/Game/Blueprint/Bateaux/Bobbie/BP_BoatTemplate` (`GameplayStatics.GetPlayerPawn` 0)))
  (set `self.Bobbie_Ref` _asbp_boat_template)
  (`self.EnableInput` (`GameplayStatics.GetPlayerController` 0)))

(event `self.BoueeSauvetage.OnComponentHit`
  (params (HitComponent :type "PrimitiveComponent Object Reference") (OtherActor :type "Actor Object Reference") (OtherComp :type "PrimitiveComponent Object Reference") (NormalImpulse :type "Vector Structure") (Hit :type "HitResult Structure (by ref)"))
  (bind (_transformationinitiale_location _transformationinitiale_rotation) (`KismetMathLibrary.BreakTransform` (`self.TransformationInitiale`)))
  ;[1 1 1] Retour à la position initial 3 secondes après l'impacte avec tout objet.
  (`KismetSystemLibrary.K2_SetTimerDelegate` (delegate `RetourPositionInitale`) 3.0)
  (goto _label :!via `Stop`))

(event `RetourPositionInitale`
  (bind (_transformationinitiale_location _transformationinitiale_rotation) (`KismetMathLibrary.BreakTransform` (`self.TransformationInitiale`)))
  ;[1 1 1] Retour à la position initial 3 secondes après l'impacte avec tout objet.
  (`self.PrintInfos` "Mouvement Naufragé:" "En cours de Déplacement " (struct :`R` 1.0 :`G` 0.958267 :`A` 1.0) 10.0)
  (`KismetSystemLibrary.MoveComponentTo` (`self.BoueeSauvetage`) (+ _transformationinitiale_location (0.0 0.0 -100.0)) _transformationinitiale_rotation true true (`self.Duree Deplacement`) :!label _label)
  (`self.PrintInfos` "Mouvement Naufragé:" "Arrivée au point de départ" (struct :`R` 0.114152 :`G` 1.0 :`A` 1.0) 10.0))

(event `self.ZoneDeRalentissement.OnComponentBeginOverlap`
  (params (OverlappedComponent :type "PrimitiveComponent Object Reference") (OtherActor :type "Actor Object Reference") (OtherComp :type "PrimitiveComponent Object Reference") (OtherBodyIndex :type Integer) (bFromSweep :type Boolean) (SweepResult :type "HitResult Structure (by ref)"))
  (bind _bobbie_ref (`self.Bobbie_Ref`))
  (if (== OtherActor (`GameplayStatics.GetPlayerPawn` 0))
    (bind _output_get (set `self.RalentissementBobbie?` true))
    (bind _output_get_2 (set `/Game/Blueprint/Bateaux/Bobbie/BP_BoatTemplate.DansLaZoneNaufrage` _output_get _bobbie_ref))
    (set `/Game/Blueprint/Bateaux/Bobbie/BP_BoatTemplate.RegardForce` _output_get_2 _bobbie_ref)
    (set `/Game/Blueprint/Bateaux/Bobbie/BP_BoatTemplate.CurrentNaufrage` self _bobbie_ref)
    (set `/Game/Blueprint/Bateaux/Bobbie/BP_BoatTemplate.RegardForce` true _bobbie_ref)
    (`/Game/Blueprint/Bateaux/Bobbie/BP_BoatTemplate.OuvrirLumiere` _bobbie_ref)
    (`/Game/Widget/WBP_UI_Jeu.DansLaZoneSauvetage` (`/Game/Blueprint/Bateaux/Bobbie/BP_BoatTemplate.UI_EnJeu` _bobbie_ref))))

(event `self.ZoneDeRalentissement.OnComponentEndOverlap`
  (params (OverlappedComponent :type "PrimitiveComponent Object Reference") (OtherActor :type "Actor Object Reference") (OtherComp :type "PrimitiveComponent Object Reference") (OtherBodyIndex :type Integer))
  (bind _bobbie_ref (`self.Bobbie_Ref`))
  (if (== OtherActor (`GameplayStatics.GetPlayerPawn` 0))
    (bind _output_get (set `self.RalentissementBobbie?` false))
    (bind _output_get_2 (set `/Game/Blueprint/Bateaux/Bobbie/BP_BoatTemplate.DansLaZoneNaufrage` _output_get _bobbie_ref))
    (set `/Game/Blueprint/Bateaux/Bobbie/BP_BoatTemplate.RegardForce` _output_get_2 _bobbie_ref)
    (set `/Game/Blueprint/Bateaux/Bobbie/BP_BoatTemplate.CurrentNaufrage` null _bobbie_ref)
    (set `/Game/Blueprint/Bateaux/Bobbie/BP_BoatTemplate.RegardForce` false _bobbie_ref)
    (`/Game/Blueprint/Bateaux/Bobbie/BP_BoatTemplate.EteindreLumiere` _bobbie_ref)
    (`/Game/Widget/WBP_UI_Jeu.PlusDansLaZoneSauvetage` (`/Game/Blueprint/Bateaux/Bobbie/BP_BoatTemplate.UI_EnJeu` _bobbie_ref))))

(event `LancerFusee`
  (bind _returnvalue (`|SpawnActorFromClass` "/Game/Blueprint/Naufrages/BP_FuseeDetresse.BP_FuseeDetresse_C" (`KismetMathLibrary.MakeTransform` (+ (`self.K2_GetActorLocation`) (0.0 0.0 100.0))) "AlwaysSpawn" "MultiplyWithRoot" null null))
  (bind _output_get (set `self.FeuDetresse_Ref` _returnvalue))
  (`/Game/Blueprint/Naufrages/BP_FuseeDetresse.GetNaufrageParent` _output_get self))

(fn `CalculForceProportionelle`
  (params (ActorEnARalentir :type "/Game/Blueprint/Bateaux/Bobbie/BP_BoatTemplate Object Reference") (Distance :type "Float (double-precision)"))
  (returns (RetourDeForce :type "Float (double-precision)"))
  (bind _datatablebateau_infos_vitessebateau (break `/Game/Blueprint/Bateaux/Bobbie/Struct_Boats` (`/Game/Blueprint/Bateaux/Bobbie/BP_BoatTemplate.DataTableBateau_Infos` ActorEnARalentir)))
  (return (* (`KismetMathLibrary.MapRangeClamped` (* (`PrimitiveComponent.GetMass` (`/Game/Blueprint/Bateaux/Bobbie/BP_BoatTemplate.SM_Bobbie` ActorEnARalentir)) (/ (`/Game/Blueprint/Bateaux/Bobbie/BP_BoatTemplate.VelociteGlobale` ActorEnARalentir) 1.0)) 0.0 (/ _datatablebateau_infos_vitessebateau 2.0) 0.0 1.0) Distance)))

(fn `NaufrageSecouru`
  (bind _bobbie_ref (`self.Bobbie_Ref`))
  (set `/Game/Blueprint/Bateaux/Bobbie/BP_BoatTemplate.IndexPersonneSecouru` (+ (`/Game/Blueprint/Bateaux/Bobbie/BP_BoatTemplate.IndexPersonneSecouru` _bobbie_ref) 1) _bobbie_ref)
  (`/Game/Widget/WBP_UI_Jeu.AjouterNaufrage` (`/Game/Blueprint/Bateaux/Bobbie/BP_BoatTemplate.UI_EnJeu` _bobbie_ref)))

(fn `PrintInfos`
  (params (NomDeValeur :type String) (Valeur :type String) (CouleurTexte :type "LinearColor Structure") (Duration :type "Float (single-precision)") (`Print À l'écran?` :type Boolean :default true))
  (`KismetSystemLibrary.PrintString` (`KismetStringLibrary.Concat_StrStr` NomDeValeur Valeur) `Print À l'écran?` true CouleurTexte Duration))

(fn `UserConstructionScript`)