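; Distress flare for a shipwreck that shows a countdown for the player's boat.
; On BeginPlay a timeline lifts the flare with random horizontal jitter, then activates its Niagara effect, starts the timer and links the timer widget.
; Tick counts down, switching the widget to a critical color in the final sixty seconds.
; At zero it disables boat movement, shows a time-out message and destroys the parent wreck.
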(event `GetNaufrageParent`
  (params (NaufrageParent :type "Actor Object Reference"))
  (set `self.Reference Naufrage Parent` NaufrageParent))

(event `self.ReceiveTick`
  (params (DeltaSeconds :type "Float (single-precision)"))
  (bind _bp_bobbie_ref (`self.BP_Bobbie_ref`))
  ;[1 1 1] Initialise le Timer une fois le feu lancé en l'air
  (if (`self.TimerLance?`)
    (bind _output_get (set `self.Compteur` (+ (`self.Compteur`) (`GameplayStatics.GetWorldDeltaSeconds`))))
    (bind _output_get_2 (set `self.Timer` (`KismetMathLibrary.Round` (- (`self.TempsMax`) _output_get))))
    (if (<= _output_get_2 0)
      (`/Engine/EditorBlueprintResources/StandardMacros.DoOnce` false
        (:`Completed`
          (`/Game/Blueprint/Bateaux/Bobbie/BP_BoatTemplate.DesactiverMouvements` _bp_bobbie_ref)
          (`/Game/Widget/WBP_UI_Jeu.MessageTempsEcoule` (`/Game/Blueprint/Bateaux/Bobbie/BP_BoatTemplate.UI_EnJeu` _bp_bobbie_ref) "Visible")
          (bind _reference_naufrage_parent (`self.Reference Naufrage Parent`)
            (:`then`
              (`self.K2_DestroyActor` _reference_naufrage_parent))
            (:`else`))))
      (elif (<= _output_get_2 60)
        (`/Engine/EditorBlueprintResources/StandardMacros.DoOnce` false
          (:`Completed`
            (`/Game/Widget/WBP_Timer.CouleurTempsCritique` (`self.TimerRef`))))))))

(event `self.ReceiveBeginPlay`
  (bind _returnvalue (`KismetMathLibrary.RandomFloatInRange` -25.0 25.0))
  (`|ExecutionSequence`
    (:`then_0`
      ;[1 1 1] Élève le feu de détresse dans les air et active le Vfx
      (bind (_direction _forcedelenvol) (`Timeline|Hauteur du feu` :!via `PlayFromStart`)
        (:`Update`
          (`SceneComponent.K2_AddRelativeLocation` (`self.Arrow`) (`KismetMathLibrary.MakeVector` _returnvalue _returnvalue (* _forcedelenvol (`self.HauteurDeLaFusee`))) false false))
        (:`Finished`
          (`ActorComponent.Activate` (`self.NS_FeuDetresse`) false)
          (set `self.TimerLance?` true)
          (`/Game/Widget/WBP_Timer.TrouverParent` (`self.TimerRef`) self))))
    (:`then_1`
      (bind _returnvalue_2 (`KismetMaterialLibrary.CreateDynamicMaterialInstance` null))
      (set `self.MaterialFusee_Ref` _returnvalue_2)
      (bind _returnvalue_3 (`|CreateWidget` "/Game/Widget/WBP_Timer.WBP_Timer_C"))
      (bind _output_get (set `self.TimerRef` _returnvalue_3))
      (`WidgetComponent.SetWidget` (`self.TempsRestant`) _output_get)
      (bind _asbp_boat_template (cast `/Game/Blueprint/Bateaux/Bobbie/BP_BoatTemplate` (`GameplayStatics.GetPlayerPawn` 0)))
      (set `self.BP_Bobbie_ref` _asbp_boat_template))))

(fn `UserConstructionScript`)