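; Template actor for a castaway the player rescues with the boat, able to launch a distress flare.
; An outer zone pushes a fast boat back with a speed-scaled force; the buoy drifts home after hits.
; The rescue zone repositions the boat facing the castaway during a blended camera cutaway with input disabled.
; It then increments the boat's rescue count, updates the UI and destroys itself and its flare.
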(event `self.ReceiveTick`
  (params (DeltaSeconds :type "Float (single-precision)"))
  (bind _bobbie_ref (`self.Bobbie_Ref`))
  (bind _returnvalue (* (`KismetMathLibrary.Normal` (- (`self.K2_GetActorLocation` _bobbie_ref) (`self.K2_GetActorLocation`))) (* (`/Game/Blueprint/Bateaux/Bobbie/BP_BoatTemplate.VelociteGlobale` _bobbie_ref) (`self.ForceRalentissement`))))
  (if (and (> (`/Game/Blueprint/Bateaux/Bobbie/BP_BoatTemplate.VelociteGlobale` (`self.Bobbie_Ref`)) 1000.0) (`self.RalentissementBobbie?`))
    (`PrimitiveComponent.AddForce` (`/Game/Blueprint/Bateaux/Bobbie/BP_BoatTemplate.SM_Bobbie` _bobbie_ref) _returnvalue "None" false)
    (`KismetSystemLibrary.PrintString` (`KismetStringLibrary.Conv_VectorToString` _returnvalue))))

(event `self.ReceiveBeginPlay`
  ;[1 1 1] Enregistrement de la position initiale
  (set `self.TransformationInitiale` (`self.GetTransform`))
  (bind _asbp_boat_template (cast `/Game/Blueprint/Bateaux/Bobbie/BP_BoatTemplate` (`GameplayStatics.GetPlayerPawn` 0)))
  (set `self.Bobbie_Ref` _asbp_boat_template))

(event `ChangementCamera`
  (bind (_relativerotation_roll _relativerotation_pitch) (`KismetMathLibrary.BreakRotator` (`SceneComponent.RelativeRotation` (`self.SpringArm`))))
  (bind (_returnvalue_x _returnvalue_y) (`KismetMathLibrary.BreakVector` (`KismetMathLibrary.Normal` (- (`SceneComponent.K2_GetComponentLocation` (`self.CineCamera`)) (`self.K2_GetActorLocation` (`self.Bobbie_Ref`))))))
  ;[1 1 1] Lancement du mouvement de caméra pour la cinématique
  (`self.DisableInput` (`self.Bobbie_Ref`) (`GameplayStatics.GetPlayerController` 0))
  (`SceneComponent.K2_SetRelativeRotation` (`self.SpringArm`) (`KismetMathLibrary.MakeRotator` _relativerotation_roll _relativerotation_pitch (`KismetMathLibrary.DegAtan2` _returnvalue_y _returnvalue_x)) false false)
  (`PlayerController.SetViewTargetWithBlend` (`GameplayStatics.GetPlayerController` 0) self 3.0 "VTBlend_EaseInOut" 2.0 false)
  (`KismetSystemLibrary.Delay` 10.0)
  (`PlayerController.SetViewTargetWithBlend` (`GameplayStatics.GetPlayerController` 0) (`GameplayStatics.GetPlayerPawn` 0) 3.0 "VTBlend_Cubic" 1.0 false)
  (`KismetSystemLibrary.Delay` 3.2)
  (`self.EnableInput` (`self.Bobbie_Ref`) (`GameplayStatics.GetPlayerController` 0))
  (`self.NaufrageSecouru`)
  (`KismetSystemLibrary.Delay` 0.25)
  (`self.K2_DestroyActor` (`self.FeuDetresse_Ref`))
  (`self.K2_DestroyActor` self))

(event `self.BoueeSauvetage.OnComponentHit`
  (params (HitComponent :type "PrimitiveComponent Object Reference") (OtherActor :type "Actor Object Reference") (OtherComp :type "PrimitiveComponent Object Reference") (NormalImpulse :type "Vector Structure") (Hit :type "HitResult Structure (by ref)"))
  (bind (_transformationinitiale_location _transformationinitiale_rotation) (`KismetMathLibrary.BreakTransform` (`self.TransformationInitiale`)))
  ;[1 1 1] Retour à la position initial 3 secondes après l'impacte avec tout objet.
  (`KismetSystemLibrary.K2_SetTimerDelegate` (delegate `RetourPositionInitale`) 3.0)
  (goto _label :!via `Stop`))

(event `RetourPositionInitale`
  (bind (_transformationinitiale_location _transformationinitiale_rotation) (`KismetMathLibrary.BreakTransform` (`self.TransformationInitiale`)))
  ;[1 1 1] Retour à la position initial 3 secondes après l'impacte avec tout objet.
  (`self.PrintInfos` "Mouvement Naufragé:" "En cours de Déplacement " (struct :`R` 1.0 :`G` 0.958267 :`A` 1.0) 10.0)
  (`KismetSystemLibrary.MoveComponentTo` (`self.BoueeSauvetage`) (+ _transformationinitiale_location (0.0 0.0 -100.0)) _transformationinitiale_rotation true true (`self.Duree Deplacement`) :!label _label)
  (`self.PrintInfos` "Mouvement Naufragé:" "Arrivée au point de départ" (struct :`R` 0.114152 :`G` 1.0 :`A` 1.0) 10.0))

(event `self.ZoneDeRecuperation.OnComponentBeginOverlap`
  (params (OverlappedComponent :type "PrimitiveComponent Object Reference") (OtherActor :type "Actor Object Reference") (OtherComp :type "PrimitiveComponent Object Reference") (OtherBodyIndex :type Integer) (bFromSweep :type Boolean) (SweepResult :type "HitResult Structure (by ref)"))
  (bind _returnvalue (`self.K2_GetActorLocation`))
  (bind _bobbie_ref (`self.Bobbie_Ref`))
  (bind _returnvalue_2 (`self.K2_GetActorLocation` _bobbie_ref))
  (bind _returnvalue_3 (`self.K2_GetActorLocation` (`self.Bobbie_Ref`)))
  ;[1 1 1] Entré dans la zone de sauvetage
  ;;[1 1 1] S'assure que c'est le joueur qui se trouve dans la zone avant d'initier la séquence.
  (if (== OtherActor (`GameplayStatics.GetPlayerPawn` 0))
    (set `self.RalentissementBobbie?` false)
    (`PrimitiveComponent.SetLinearDamping` (`/Game/Blueprint/Bateaux/Bobbie/BP_BoatTemplate.SM_Bobbie` (`self.Bobbie_Ref`)) 2.0)
    (`ActorComponent.K2_DestroyComponent` (`self.Niagara`))
    ;;[1 1 1] Initialise le mouvement ed caméra pour la cinématique
    (`self.ChangementCamera`)
    ;;[1 1 1] En cours - Positionnement automatique du bateau à un endroit précis  -  ***Voir s'il n'est pas possible de controler le bateau à partir d'un AI controller utilisant les contrôle prédéfini
    (bind _outhit (`KismetSystemLibrary.LineTraceSingle` :`Start` (+ _returnvalue_3 (0.0 0.0 500.0)) :`End` (- _returnvalue_3 (0.0 0.0 1000.0)) :`TraceChannel` "TraceTypeQuery1" :`DrawDebugType` "ForDuration" :`DrawTime` 10.0))
    (`KismetSystemLibrary.MoveComponentTo` (`/Game/Blueprint/Bateaux/Bobbie/BP_BoatTemplate.SM_Bobbie` _bobbie_ref) (`KismetMathLibrary.MakeVector` (.x (+ (* 1000.0 (`KismetMathLibrary.Normal` (- _returnvalue_2 _returnvalue))) _returnvalue)) (.y (+ (* 1000.0 (`KismetMathLibrary.Normal` (- _returnvalue_2 _returnvalue))) _returnvalue)) (.z (`.ImpactPoint` (`GameplayStatics.BreakHitResult` _outhit)))) (`KismetMathLibrary.FindLookAtRotation` _returnvalue_2 _returnvalue) true true 3.0)
    (`PrimitiveComponent.SetLinearDamping` (`/Game/Blueprint/Bateaux/Bobbie/BP_BoatTemplate.SM_Bobbie` (`self.Bobbie_Ref`)) 0.0)))

(event `self.ZoneDeRecuperation.OnComponentEndOverlap`
  (params (OverlappedComponent :type "PrimitiveComponent Object Reference") (OtherActor :type "Actor Object Reference") (OtherComp :type "PrimitiveComponent Object Reference") (OtherBodyIndex :type Integer))
  (bind _returnvalue (`GameplayStatics.GetPlayerPawn` 0))
  (if (== OtherActor _returnvalue)
    (cast `/Game/Blueprint/Bateaux/Bobbie/BP_BoatTemplate` _returnvalue)))

(event `self.ZoneDeRalentissement.OnComponentBeginOverlap`
  (params (OverlappedComponent :type "PrimitiveComponent Object Reference") (OtherActor :type "Actor Object Reference") (OtherComp :type "PrimitiveComponent Object Reference") (OtherBodyIndex :type Integer) (bFromSweep :type Boolean) (SweepResult :type "HitResult Structure (by ref)"))
  (if (== OtherActor (`GameplayStatics.GetPlayerPawn` 0))
    (set `self.RalentissementBobbie?` true)))

(event `self.ZoneDeRalentissement.OnComponentEndOverlap`
  (params (OverlappedComponent :type "PrimitiveComponent Object Reference") (OtherActor :type "Actor Object Reference") (OtherComp :type "PrimitiveComponent Object Reference") (OtherBodyIndex :type Integer))
  (if (== OtherActor (`GameplayStatics.GetPlayerPawn` 0))
    (set `self.RalentissementBobbie?` false)))

(event `LancerFusee`
  (bind _returnvalue (`|SpawnActorFromClass` "/Game/Blueprint/Naufrages/BP_FuseeDetresse.BP_FuseeDetresse_C" (`KismetMathLibrary.MakeTransform` (+ (`self.K2_GetActorLocation`) (0.0 0.0 100.0))) "AlwaysSpawn" "MultiplyWithRoot" null null))
  (bind _output_get (set `self.FeuDetresse_Ref` _returnvalue))
  (`/Game/Blueprint/Naufrages/BP_FuseeDetresse.GetNaufrageParent` _output_get self))

(fn `NaufrageSecouru`
  (bind _bobbie_ref (`self.Bobbie_Ref`))
  (set `/Game/Blueprint/Bateaux/Bobbie/BP_BoatTemplate.IndexPersonneSecouru` (+ (`/Game/Blueprint/Bateaux/Bobbie/BP_BoatTemplate.IndexPersonneSecouru` _bobbie_ref) 1) _bobbie_ref)
  (`/Game/Widget/WBP_UI_Jeu.AjouterNaufrage` (`/Game/Blueprint/Bateaux/Bobbie/BP_BoatTemplate.UI_EnJeu` _bobbie_ref)))

(fn `PrintInfos`
  (params (NomDeValeur :type String) (Valeur :type String) (CouleurTexte :type "LinearColor Structure") (Duration :type "Float (single-precision)") (`Print À l'écran?` :type Boolean :default true))
  (`KismetSystemLibrary.PrintString` (`KismetStringLibrary.Concat_StrStr` NomDeValeur Valeur) `Print À l'écran?` true CouleurTexte Duration))

(fn `UserConstructionScript`)