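; Lifebuoy actor running a timing minigame to rescue the boat's current shipwreck.
; A timeline slides the buoy along a gauge placed at the wreck, while Tick feeds a three-point Niagara aiming line.
; Throwing inside the ideal overlap zone switches the hologram material, stops the buoy, repossesses the boat, then removes and counts the wreck after a delay.
; A miss only updates text; cancel repossesses the boat.
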(event `self.ReceiveTick`
  (params (DeltaSeconds :type "Float (single-precision)"))
  (bind _positiontrajectoire (`self.PositionTrajectoire`))
  (bind _returnvalue (`KismetMathLibrary.Vector_Distance` (`SceneComponent.K2_GetComponentLocation` (`self.StaticMesh`)) (`self.K2_GetActorLocation` (`self.As BP Boat Template`))))
  (bind _returnvalue_2 (* _returnvalue -1.0))
  (`/Engine/EditorBlueprintResources/StandardMacros.IsValid` (`self.As BP Boat Template`)
    (:`Is Valid`
      (`KismetArrayLibrary.Array_Set` _positiontrajectoire)
      (`KismetArrayLibrary.Array_Set` _positiontrajectoire 1 (`KismetMathLibrary.MakeVector` 0.0 (/ _returnvalue_2 2.0) (/ _returnvalue 2.0)))
      (`KismetArrayLibrary.Array_Set` _positiontrajectoire 2 (`KismetMathLibrary.MakeVector` 0.0 _returnvalue_2))
      (`NiagaraDataInterfaceArrayFunctionLibrary.SetNiagaraArrayVector` (`self.AimingLine `) "User.PositionParticules" _positiontrajectoire))))

(event `self.ReceiveBeginPlay`
  (bind _returnvalue (`GameplayStatics.GetActorOfClass` "/Game/Blueprint/Bateaux/Bobbie/BP_BoatTemplate.BP_BoatTemplate_C"))
  (set `self.As BP Boat Template` _returnvalue)
  ;[1 1 1] Place la jauge à l'emplacement du naufrage
  (`SceneComponent.K2_SetWorldLocation` (`self.AimingWidget`) (+ (`self.K2_GetActorLocation` (`/Game/Blueprint/Bateaux/Bobbie/BP_BoatTemplate.CurrentNaufrage` (`self.As BP Boat Template`))) (0.0 0.0 40.0)) false false)
  (`KismetSystemLibrary.Delay` 0.2)
  (`self.EnableInput` (`GameplayStatics.GetPlayerController` 0))
  (bind _returnvalue_2 (`PrimitiveComponent.CreateDynamicMaterialInstance` (`self.StaticMesh`) 0 "/Game/Material/Instances/MI_BoueeSauvetage.MI_BoueeSauvetage" "None"))
  (bind _output_get (set `self.MaterailBouee` _returnvalue_2))
  (`MaterialInstanceDynamic.SetScalarParameterValue` _output_get "HologramTransition" 0.0)
  (`self.Go`))

(event `CancelShot`
  (`self.K2_DestroyActor` :!label _label))

(event `EnhancedInput|/Game/Controls/Inputs/ControleBouee/IA_Lancer`
  (params (ActionValue :type Boolean) (ElapsedSeconds :type "Float (double-precision)") (TriggeredSeconds :type "Float (double-precision)") (InputAction :type "InputAction Object Reference" :default "/Game/Controls/Inputs/ControleBouee/IA_Lancer.IA_Lancer"))
  (:`Started`
    (if (`self.TirReussi`)
      (`MaterialInstanceDynamic.SetScalarParameterValue` (`self.MaterailBouee`) "HologramTransition" 1.0)
      (`self.StopMouvement `)
      (`|ExecutionSequence`
        (:`then_0`
          (`KismetSystemLibrary.Delay` 1.2)
          (`self.K2_DestroyActor` (`/Game/Blueprint/Bateaux/Bobbie/BP_BoatTemplate.CurrentNaufrage` (`self.As BP Boat Template`)))
          (`/Game/Widget/WBP_UI_Jeu.AjouterNaufrage` (`/Game/Blueprint/Bateaux/Bobbie/BP_BoatTemplate.UI_EnJeu` (`self.As BP Boat Template`)))
          (goto _label))
        (:`then_1`
          (`/Game/Blueprint/Bateaux/Bobbie/BP_BoatTemplate.Repossess` (`self.As BP Boat Template`) false)))
      (else
        (`TextRenderComponent.K2_SetText` (`self.TextRender`) (`self.Value`))))))

(event `EnhancedInput|/Game/Controls/Inputs/ControleBateau/IA_Cancel-Back`
  (params (ActionValue :type Boolean) (ElapsedSeconds :type "Float (double-precision)") (TriggeredSeconds :type "Float (double-precision)") (InputAction :type "InputAction Object Reference" :default "/Game/Controls/Inputs/ControleBateau/IA_Cancel-Back.IA_Cancel-Back"))
  (:`Started`
    (`/Game/Blueprint/Bateaux/Bobbie/BP_BoatTemplate.Repossess` (`self.As BP Boat Template`) true)))

(event `Go`
  ;[1 1 1] Mouvement de la bouee sur la jaug, pssibilité de set uune new curve afin de varier l'intensité, la vitesse ainsi que la difficulté.
  (if (`self.Avance-Recule`)
    (bind (_direction _vitessejauge) (`Timeline|CadenceLancer` :!via `PlayFromStart` :!label _label_2)
      (:`Update`
        (bind _returnvalue (* _vitessejauge 35.0))
        (`SceneComponent.K2_AddLocalOffset` (`self.StaticMesh`) (`KismetMathLibrary.MakeVector` (`KismetMathLibrary.SelectFloat` (* _returnvalue -1.0) _returnvalue (`self.Avance-Recule`))) false false))
      (:`Finished`
        (if (`self.Avance-Recule`)
          (set `self.Avance-Recule` false)
          (else
            (set `self.Avance-Recule` true)))
        (`self.Go`)))
    (else
      (goto _label_2 :!via `ReverseFromEnd`))))

(event `StopMouvement`
  ;[1 1 1] Mouvement de la bouee sur la jaug, pssibilité de set uune new curve afin de varier l'intensité, la vitesse ainsi que la difficulté.
  (goto _label_2 :!via `Stop`))

(event `self.ZoneIdeal.OnComponentBeginOverlap`
  (params (OverlappedComponent :type "PrimitiveComponent Object Reference") (OtherActor :type "Actor Object Reference") (OtherComp :type "PrimitiveComponent Object Reference") (OtherBodyIndex :type Integer) (bFromSweep :type Boolean) (SweepResult :type "HitResult Structure (by ref)"))
  ;[1 1 1] Comment
  (`KismetSystemLibrary.PrintString` (`KismetStringLibrary.Concat_StrStr` "In:" (`KismetSystemLibrary.GetDisplayName` OtherComp)) true true (struct :`R` 0.279682 :`G` 1.0 :`A` 1.0) 60.0)
  (if (or (== OtherComp (`self.Cible`)) (== (`self.StaticMesh`) OtherComp))
    (set `self.TirReussi` true)))

(event `self.ZoneIdeal.OnComponentEndOverlap`
  (params (OverlappedComponent :type "PrimitiveComponent Object Reference") (OtherActor :type "Actor Object Reference") (OtherComp :type "PrimitiveComponent Object Reference") (OtherBodyIndex :type Integer))
  (`KismetSystemLibrary.PrintString` (`KismetStringLibrary.Concat_StrStr` "Out: " (`KismetSystemLibrary.GetDisplayName` OtherComp)) true true (struct :`R` 1.0 :`G` 0.022333 :`A` 1.0) 60.0)
  (if (or (== OtherComp (`self.Cible`)) (== (`self.StaticMesh`) OtherComp))
    (set `self.TirReussi` false)))

(fn `UserConstructionScript`)