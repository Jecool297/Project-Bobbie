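; Boat template Blueprint that drives a physics-simulated, buoyant static mesh from Enhanced Input throttle, reverse and steering actions.
; While the Buoyancy component is in a water body, each action applies an offset local force that scales with clamped hold time and the boat's speed or turn strength.
; Debug prints show forward vector and velocity, T applies a test torque, and a velocity-based vertical force is left unconnected.
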(event Input|EnhancedActionEvents|EnhancedInputActionIA_SteerLeft
  (params (ActionValue :type Boolean) (ElapsedSeconds :type Float%20%28double-precision%29) (TriggeredSeconds :type Float%20%28double-precision%29) (InputAction :type Input%20Action%20Object%20Reference :default "/Game/Controls/Inputs/IA_SteerLeft.IA_SteerLeft"))
  ;[1 1 1] Rotation vers la gauche à l'appui du input correspndant.
  (if (Buoyancy|IsinWaterBody (Variables|Default|GetBuoyancy))
    (Class|PrimitiveComponent|AddForceatLocationLocal (Variables|Default|GetStaticMesh) (Math|Vector|MakeVector (* (Math|Float|Clamp(Float) TriggeredSeconds 0.5 3.0) (Variables|Default|GetBoatTurnStrenght)) 0.0 0.0) "0.000000,200.000000,0.000000" "None")))

(event Input|EnhancedActionEvents|EnhancedInputActionIA_SteerRight
  (params (ActionValue :type Boolean) (ElapsedSeconds :type Float%20%28double-precision%29) (TriggeredSeconds :type Float%20%28double-precision%29) (InputAction :type Input%20Action%20Object%20Reference :default "/Game/Controls/Inputs/IA_SteerRight.IA_SteerRight"))
  ;[1 1 1] Rotation vers la droite à l'appui du input correspndant.
  (:Triggered
    (if (Buoyancy|IsinWaterBody (Variables|Default|GetBuoyancy))
      (Class|PrimitiveComponent|AddForceatLocationLocal (Variables|Default|GetStaticMesh) (Math|Vector|MakeVector (* (Math|Float|Clamp(Float) TriggeredSeconds 0.5 3.0) (* (Variables|Default|GetBoatTurnStrenght) -1.0)) 0.0 0.0) "0.000000,250.000000,100.000000" "None"))))

(event Input|EnhancedActionEvents|EnhancedInputActionIA_Throttle
  (params (ActionValue :type Float%20%28double-precision%29) (ElapsedSeconds :type Float%20%28double-precision%29) (TriggeredSeconds :type Float%20%28double-precision%29) (InputAction :type Input%20Action%20Object%20Reference :default "/Game/Controls/Inputs/IA_Throttle.IA_Throttle"))
  (bind _staticmesh (Variables|Default|GetStaticMesh))
  (if (Buoyancy|IsinWaterBody (Variables|Default|GetBuoyancy))
    (Class|PrimitiveComponent|AddForceatLocationLocal (Variables|Default|GetStaticMesh) (Math|Vector|MakeVector 0.0 (* ActionValue (* (Math|Float|Clamp(Float) TriggeredSeconds 0.0 3.0) (Variables|Default|GetBoatSpeed))) 0.0) (Math|Vector|MakeVector 0.0 (* ActionValue 3e+02) 0.0) "None")
    ;[1 1 1] Poussée ver le haut lorsque l'on avance
    (CallFunction|PrintInfos "Forward Vector " (Utilities|String|ToString(Vector) (Math|Vector|GetForwardVector _staticmesh)) "(R=1.000000,G=0.973697,B=0.000000,A=1.000000)" 0.0)
    (CallFunction|PrintInfos "Velocite" (Utilities|String|ToString(Vector) (Transformation|GetComponentVelocity _staticmesh)) "(R=1.000000,G=0.453811,B=0.000000,A=1.000000)" 0.0)))

(event Input|EnhancedActionEvents|EnhancedInputActionIA_Reverse
  (params (ActionValue :type Boolean) (ElapsedSeconds :type Float%20%28double-precision%29) (TriggeredSeconds :type Float%20%28double-precision%29) (InputAction :type Input%20Action%20Object%20Reference :default "/Game/Controls/Inputs/IA_Reverse.IA_Reverse"))
  ;[1 1 1] S'assure que le bateau est dans l'eau
  (if (Buoyancy|IsinWaterBody (Variables|Default|GetBuoyancy))
    (Class|PrimitiveComponent|AddForceatLocationLocal (Variables|Default|GetStaticMesh) (Math|Vector|MakeVector 0.0 (* (* (Math|Float|Clamp(Float) TriggeredSeconds 0.0 3.0) (Variables|Default|GetBoatSpeed)) -1.0) 0.0) "0.000000,100.000000,0.000000" "None")))

(event EventBeginPlay)

(event Collision|EventActorBeginOverlap
  (params (OtherActor :type Actor%20Object%20Reference)))

(event EventTick
  (params (DeltaSeconds :type Float%20%28single-precision%29)))

(event Input|KeyboardEvents|DebugKeyT
  (params (Key :type Key%20Structure :default "None") (ActionValue :type Input%20Action%20Value%20Structure))
  (:Pressed
    (Class|PrimitiveComponent|AddTorqueinDegrees (Variables|Default|GetStaticMesh) "110000.000000,0.000000,0.000000" "None" false)))

(fn ConstructionScript)

(fn PrintInfos
  (params (Nom%20de%20la%20valeur :type String) (Valeur :type String) (Couleur%20du%20texte :type Linear%20Color%20Structure) (Duration :type Float%20%28single-precision%29))
  (Development|PrintString (Utilities|String|Append Nom%20de%20la%20valeur Valeur) true true Couleur%20du%20texte Duration))