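; Water current zone that repels the player's boat (BP_BoatTemplate) away from its Arrow component.
; The construction script sizes a sphere trigger to TailleCourant, and its overlap events store or clear the boat reference.
; While the boat is inside, Tick pushes its mesh with a force scaled by ForceDuCourant and a clamped remap of distance.
; Tick also prints that distance on screen for debugging.
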(event `self.ReceiveTick`
  (params (DeltaSeconds :type "Float (single-precision)"))
  (bind _taillecourant (`self.TailleCourant`))
  (bind _returnvalue (`SceneComponent.K2_GetComponentLocation` (`self.Arrow`)))
  (bind _sm_bobbie (`/Game/Blueprint/Bateaux/Bobbie/BP_BoatTemplate.SM_Bobbie` (`self.Bobbie_Ref`)))
  (bind _returnvalue_2 (`SceneComponent.K2_GetComponentLocation` _sm_bobbie))
  (bind _returnvalue_3 (`KismetMathLibrary.Vector_Distance` _returnvalue _returnvalue_2))
  (if (`self.JoueurDansLeCourant?`)
    (`KismetSystemLibrary.PrintString` (`KismetStringLibrary.Concat_StrStr` "Distance:" (`KismetStringLibrary.Conv_DoubleToString` _returnvalue_3)) true true (struct :`R` 1.0 :`B` 0.469434 :`A` 1.0))
    (`PrimitiveComponent.AddForce` _sm_bobbie (* (`KismetMathLibrary.Normal` (- _returnvalue _returnvalue_2)) (* (* (`KismetMathLibrary.MapRangeClamped` (- _taillecourant _returnvalue_3) 100.0 _taillecourant 5000.0) (`self.ForceDuCourant`)) -1.0)) "None" false)))

(event `self.Sphere1.OnComponentBeginOverlap`
  (params (OverlappedComponent :type "PrimitiveComponent Object Reference") (OtherActor :type "Actor Object Reference") (OtherComp :type "PrimitiveComponent Object Reference") (OtherBodyIndex :type Integer) (bFromSweep :type Boolean) (SweepResult :type "HitResult Structure (by ref)"))
  ;[1 1 1] Détecte l'entrée du joueur dans la zone du courant
  (if (== OtherActor (`GameplayStatics.GetPlayerPawn` 0))
    (bind _asbp_boat_template (cast `/Game/Blueprint/Bateaux/Bobbie/BP_BoatTemplate` OtherActor))
    (set `self.Bobbie_Ref` _asbp_boat_template)
    (set `self.JoueurDansLeCourant?` true)))

(event `self.Sphere1.OnComponentEndOverlap`
  (params (OverlappedComponent :type "PrimitiveComponent Object Reference") (OtherActor :type "Actor Object Reference") (OtherComp :type "PrimitiveComponent Object Reference") (OtherBodyIndex :type Integer))
  ;[1 1 1] Détecte la sortie du joueur de la zone de courant
  (if (== OtherActor (`GameplayStatics.GetPlayerPawn` 0))
    (set `self.JoueurDansLeCourant?` false)
    (set `self.Bobbie_Ref` null)))

(fn `UserConstructionScript`
  (`SphereComponent.SetSphereRadius` (`self.Sphere1`) (`self.TailleCourant`) true))