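; BP_CourantEau is a water current volume, still in progress, intended to push the player's boat.
; The construction script sizes its Box from TailleCourant, and overlap events store or clear the BP_BoatTemplate reference.
; While the boat is inside, Tick prints its distance from the Arrow and a range-mapped value.
; AddForce currently applies a zero vector, as the ForceDuCourant scaling is left unconnected.
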(event `self.ReceiveTick`
  (params (DeltaSeconds :type "Float (single-precision)"))
  (bind _sm_bobbie (`/Game/Blueprint/Bateaux/BP_BoatTemplate.SM_Bobbie` (`self.Bobbie_Ref`)))
  (bind _returnvalue (`KismetMathLibrary.Vector_Distance` (`SceneComponent.K2_GetComponentLocation` (`self.Arrow`)) (`SceneComponent.K2_GetComponentLocation` _sm_bobbie)))
  (if (`self.JoueurDansLeCourant?`)
    (`KismetSystemLibrary.PrintString` (`KismetStringLibrary.Concat_StrStr` "Distance Dynamiqu e: " (`KismetStringLibrary.Conv_DoubleToString` (`KismetMathLibrary.MapRangeClamped` (- (.x (`.BoxExtent` (`KismetSystemLibrary.GetComponentBounds` (`self.Box`)))) _returnvalue) -3000.0 -1000.0 1000.0 5000.0))) true true (struct :`G` 1.0 :`B` 0.289114 :`A` 1.0))
    (`KismetSystemLibrary.PrintString` (`KismetStringLibrary.Concat_StrStr` "Distance:" (`KismetStringLibrary.Conv_DoubleToString` _returnvalue)) true true (struct :`R` 1.0 :`B` 0.469434 :`A` 1.0))
    (`PrimitiveComponent.AddForce` _sm_bobbie (0.0 0.0 0.0) "None" false)))

(event `self.Box.OnComponentBeginOverlap`
  (params (OverlappedComponent :type "PrimitiveComponent Object Reference") (OtherActor :type "Actor Object Reference") (OtherComp :type "PrimitiveComponent Object Reference") (OtherBodyIndex :type Integer) (bFromSweep :type Boolean) (SweepResult :type "HitResult Structure (by ref)"))
  ;[1 1 1] Détecte l'entrée du joueur dans la zone du courant
  (if (== OtherActor (`GameplayStatics.GetPlayerPawn` 0))
    (bind _asbp_boat_template (cast `/Game/Blueprint/Bateaux/BP_BoatTemplate` OtherActor))
    (set `self.Bobbie_Ref` _asbp_boat_template)
    (set `self.JoueurDansLeCourant?` true)))

(event `self.Box.OnComponentEndOverlap`
  (params (OverlappedComponent :type "PrimitiveComponent Object Reference") (OtherActor :type "Actor Object Reference") (OtherComp :type "PrimitiveComponent Object Reference") (OtherBodyIndex :type Integer))
  ;[1 1 1] Détecte la sortie du joueur de la zone de courant
  (if (== OtherActor (`GameplayStatics.GetPlayerPawn` 0))
    (set `self.JoueurDansLeCourant?` false)
    (set `self.Bobbie_Ref` null)))

(fn `UserConstructionScript`
  (`BoxComponent.SetBoxExtent` (`self.Box`) (`self.TailleCourant`) true))