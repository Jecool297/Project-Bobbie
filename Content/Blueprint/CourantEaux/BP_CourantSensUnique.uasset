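; One-way water current volume that pushes the player's boat (Bobbie) along the actor's forward vector.
; Box, sized by TailleCourant in construction, tracks the player's BP_BoatTemplate on overlap, and Tick applies AddForce to its mesh.
; Force grows near the Arrow; heading upstream scales it by boat velocity, boosted above a threshold, otherwise MultiplicateurDansLeCourant applies.
; Tick also prints debug values on screen.
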(event `self.ReceiveBeginPlay`)

(event `self.ReceiveTick`
  (params (DeltaSeconds :type "Float (single-precision)"))
  (bind _velocitelocale_x (`KismetMathLibrary.BreakVector` (`/Game/Blueprint/Bateaux/Bobbie/BP_BoatTemplate.VelociteLocale` (`self.Bobbie_Ref`))))
  (bind _velocitelocale_x_2 (`KismetMathLibrary.BreakVector` (`/Game/Blueprint/Bateaux/Bobbie/BP_BoatTemplate.VelociteLocale` (`self.Bobbie_Ref`))))
  (bind _sm_bobbie (`/Game/Blueprint/Bateaux/Bobbie/BP_BoatTemplate.SM_Bobbie` (`self.Bobbie_Ref`)))
  (bind _returnvalue (`KismetMathLibrary.Vector_Distance` (`SceneComponent.K2_GetComponentLocation` (`self.Arrow`)) (`SceneComponent.K2_GetComponentLocation` _sm_bobbie)))
  (bind _returnvalue_2 (< (`KismetMathLibrary.Dot_VectorVector` (`self.GetActorForwardVector`) (`SceneComponent.GetForwardVector` _sm_bobbie)) 0.0))
  (bind _returnvalue_3 (`KismetMathLibrary.MapRangeClamped` (- (* (.x (`.BoxExtent` (`KismetSystemLibrary.GetComponentBounds` (`self.Box`)))) 2.0) _returnvalue) 0.0 10000.0 10.0 100.0))
  (bind _returnvalue_4 (* (* _returnvalue_3 (`KismetMathLibrary.SelectFloat` _velocitelocale_x_2 (`KismetMathLibrary.Abs` _velocitelocale_x_2) (> _velocitelocale_x_2 0.0))) (`self.ForceDuCourant`)))
  (bind _returnvalue_5 (* 1.0 (`KismetMathLibrary.SelectFloat` (`KismetMathLibrary.SelectFloat` (* _returnvalue_4 4.0) _returnvalue_4 (> _returnvalue_3 50.0)) (* (* _returnvalue_3 (`self.ForceDuCourant`)) (`self.MultiplicateurDansLeCourant`)) (and _returnvalue_2 (> _velocitelocale_x 0.0)))))
  (bind _returnvalue_6 (* (`self.GetActorForwardVector`) _returnvalue_5))
  (`|ExecutionSequence`
    (:`then_0`
      (`KismetSystemLibrary.PrintString` (`KismetStringLibrary.Concat_StrStr` "Vagues" (`KismetSystemLibrary.GetDisplayName` null))))
    (:`then_1`
      (if (`self.JoueurDansLeCourant?`)
        ;[1 1 1] Calcul de la distance entre Bobbie et l'extrémité du courant dépendamment de la taille du courant afin d'appliquer une force adapté. Inversion par *-1 pour appliquer la force à l'arrière du bateau
        (`KismetSystemLibrary.PrintString` (`KismetStringLibrary.Concat_StrStr` (`KismetStringLibrary.Concat_StrStr` (`KismetStringLibrary.Conv_DoubleToString` _returnvalue_3) "Est ") (`KismetStringLibrary.Conv_BoolToString` _returnvalue_2)) true true (struct :`R` 0.204838 :`G` 1.0 :`A` 1.0) 50.0)
        ;[1 1 1] Print d'informations
        (`self.PrintInfos` "Direction et force du courant : " (`KismetStringLibrary.Conv_VectorToString` _returnvalue_6) (struct :`R` 1.0 :`B` 0.985553 :`A` 1.0))
        (`self.PrintInfos` "Force dynamique du courant actuel" (`KismetStringLibrary.Conv_DoubleToString` _returnvalue_5) (struct :`R` 1.0 :`B` 0.752942 :`A` 1.0))
        (`self.PrintInfos` "Distance Entre le courant et le bateau:" (`KismetStringLibrary.Conv_DoubleToString` _returnvalue) (struct :`R` 1.0 :`B` 0.752942 :`A` 1.0))
        ;[1 1 1] Ajout de la force à l'arrière de Bobbie dans la direction du courant lorsqu'il est à sens inverse
        (`PrimitiveComponent.AddForce` _sm_bobbie _returnvalue_6 "None" false)))))

(event `self.Box.OnComponentBeginOverlap`
  (params (OverlappedComponent :type "PrimitiveComponent Object Reference") (OtherActor :type "Actor Object Reference") (OtherComp :type "PrimitiveComponent Object Reference") (OtherBodyIndex :type Integer) (bFromSweep :type Boolean) (SweepResult :type "HitResult Structure (by ref)"))
  ;[1 1 1] Détecte l'entrée du joueur dans la zone du courant
  (if (== OtherActor (`GameplayStatics.GetPlayerPawn` 0))
    (bind _asbp_boat_template (cast `/Game/Blueprint/Bateaux/Bobbie/BP_BoatTemplate` OtherActor))
    (set `self.Bobbie_Ref` _asbp_boat_template)
    (set `self.JoueurDansLeCourant?` true)))

(event `self.Box.OnComponentEndOverlap`
  (params (OverlappedComponent :type "PrimitiveComponent Object Reference") (OtherActor :type "Actor Object Reference") (OtherComp :type "PrimitiveComponent Object Reference") (OtherBodyIndex :type Integer))
  ;[1 1 1] Détecte la sortie du joueur de la zone de courant
  (if (== OtherActor (`GameplayStatics.GetPlayerPawn` 0))
    (set `self.JoueurDansLeCourant?` false)
    (set `self.Bobbie_Ref` null)))

(fn `PrintInfos`
  (params (`Nom de la valeur` :type String) (Valeur :type String) (`Couleur du texte` :type "LinearColor Structure") (Duration :type "Float (single-precision)") (`PrintToScreen?` :type Boolean :default true))
  (`KismetSystemLibrary.PrintString` (`KismetStringLibrary.Concat_StrStr` `Nom de la valeur` Valeur) `PrintToScreen?` true `Couleur du texte` Duration))

(fn `UserConstructionScript`
  (`BoxComponent.SetBoxExtent` (`self.Box`) (`self.TailleCourant`) true))