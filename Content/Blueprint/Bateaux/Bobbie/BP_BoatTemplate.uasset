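; Player boat template whose type selects mesh and data-table handling stats in the construction script.
; Throttle, brake and steering apply local forces while buoyancy reports water contact, with AI entry points and a Tick counter-force against sideslip.
; Spring-arm camera offers mouse/gamepad look, delayed recentering, first/third-person toggle and speed-based FOV.
; Impacts trigger rumble, speed-scaled damage to health and UI, and temporary immunity; the forced flare-focus camera is unfinished.
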(event `self.ReceiveBeginPlay`
  (bind _returnvalue (`|CreateWidget` "/Game/Widget/WBP_UI_Jeu.WBP_UI_Jeu_C"))
  (bind _output_get (set `self.UI_EnJeu` _returnvalue))
  (`UserWidget.AddToViewport` _output_get 0))

(event `self.ReceiveTick`
  (params (DeltaSeconds :type "Float (single-precision)"))
  (bind (_velocitelocale_x _velocitelocale_y) (`KismetMathLibrary.BreakVector` (`self.VelociteLocale`)))
  (bind _velocitelocale_x_2 (`KismetMathLibrary.BreakVector` (`self.VelociteLocale`)))
  (bind _returnvalue (* _velocitelocale_y -100.0))
  ;[1 1 1] Gestion  de la contre force appliqué sur le bateau lorsque l'on tourne.
  (set `self.VelociteLocale` (`KismetMathLibrary.InverseTransformDirection` (`self.GetTransform`) (`self.GetVelocity`)))
  (set `self.VelociteGlobale` (`KismetMathLibrary.VSize` (`self.GetVelocity`)))
  (`|ExecutionSequence`
    (:`then_0`
      (if (`self.RegardForce`)
        (`self.FocusNaufrage`)
        (elif (not (`self.ControleDeCamera?`))
          (`SceneComponent.K2_SetRelativeRotation` (`self.SpringArm`) (`KismetMathLibrary.RInterpTo` (`SceneComponent.RelativeRotation` (`self.SpringArm`)) (`SceneComponent.RelativeRotation` (`self.OrientationCamera`)) (`GameplayStatics.GetWorldDeltaSeconds`) 0.5) false false))))
    (:`then_1`
      (`self.AjustementFieldOfView`))
    (:`then_2`
      (if (<= _velocitelocale_x_2 -1000.0)
        (`self.Freinage_AI`)
        (else
          (set `self.Freinage_IA` false))))
    (:`then_3`
      ;;[1 1 1] Effectue un calcul de contre force en transférant la vélocité de bobbie comme force opposé au coté latérale en question
      (bind (_contre_force _glissement_) (`self.CalculContreForceLateral`))
      (if (and _glissement_ (`BuoyancyComponent.IsInWaterBody` (`self.Buoyancy1`)))
        (`PrimitiveComponent.AddForceAtLocationLocal` (`self.SM_Bobbie`) (`KismetMathLibrary.MakeVector` (* _velocitelocale_x 2.0) _returnvalue) (0.0 0.0 0.0) "None")
        (`self.Print_Infos` "Force de poussé" (`KismetStringLibrary.Conv_DoubleToString` _returnvalue) (struct :`G` 1.0 :`B` 0.364774 :`A` 1.0))))))

(event `EnhancedInput|/Game/Controls/Inputs/IA_LookAroundController`
  (params (ActionValue :type "Vector2D Structure") (ElapsedSeconds :type "Float (double-precision)") (TriggeredSeconds :type "Float (double-precision)") (InputAction :type "InputAction Object Reference" :default "/Game/Controls/Inputs/IA_LookAroundController.IA_LookAroundController"))
  (bind _sensibilitevue (`self.SensibiliteVue`))
  (bind (_relativerotation_roll _relativerotation_pitch _relativerotation_yaw) (`KismetMathLibrary.BreakRotator` (`SceneComponent.RelativeRotation` (`self.SpringArm`))))
  ;[1 1 1] Controle de la caméra avec souris et manette
  ;;[1 1 1] Mouvements et limitations de la caméra à la manette
  (:`Triggered`
    (set `self.ControleDeCamera?` true)
    (`SceneComponent.K2_SetRelativeRotation` (`self.SpringArm`) (`KismetMathLibrary.RInterpTo` (`SceneComponent.RelativeRotation` (`self.SpringArm`)) (`KismetMathLibrary.MakeRotator` 0.0 (`KismetMathLibrary.FClamp` (+ (* (* ActionValue_Y _sensibilitevue) -1.0) _relativerotation_pitch) (`self.VueMinimum_Y`) (`self.VueMaximum_Y`)) (`KismetMathLibrary.FClamp` (+ (* ActionValue_X _sensibilitevue) _relativerotation_yaw) (`self.VueMinimum_X`) (`self.VueMaximum_X`))) (`GameplayStatics.GetWorldDeltaSeconds`) 15.0) false false))
  (:`Canceled`
    (`KismetSystemLibrary.Delay` (`self.DelaiRepositionnementCamera`) :!label _label)
    (set `self.ControleDeCamera?` false))
  (:`Completed`
    (goto _label)))

(event `AjustementFieldOfView`
  (bind _velocitelocale_x (`KismetMathLibrary.BreakVector` (`self.VelociteLocale`)))
  (bind _fovmaximum (`self.FOVMaximum`))
  ;[1 1 1] Ajuste le field of view en fonction de la vitesse du bateau pour donner une impression de vitesse
  (`CameraComponent.SetFieldOfView` (`self.Camera`) (`KismetMathLibrary.MapRangeClamped` _velocitelocale_x 500.0 1500.0 (`self.FOVMinimum`) (`KismetMathLibrary.SelectFloat` (+ _fovmaximum 30.0) _fovmaximum (`self.DansLeCourant?`)))))

(event `EnhancedInput|/Game/Controls/Inputs/IA_LookAroundMouse`
  (params (ActionValue :type "Vector2D Structure") (ElapsedSeconds :type "Float (double-precision)") (TriggeredSeconds :type "Float (double-precision)") (InputAction :type "InputAction Object Reference" :default "/Game/Controls/Inputs/IA_LookAroundMouse.IA_LookAroundMouse"))
  (bind _sensibilitevue (`self.SensibiliteVue`))
  (bind (_relativerotation_roll _relativerotation_pitch _relativerotation_yaw) (`KismetMathLibrary.BreakRotator` (`SceneComponent.RelativeRotation` (`self.SpringArm`))))
  ;[1 1 1] Controle de la caméra avec souris et manette
  ;;[1 1 1] Mouvements et limitations de la caméra à la souris
  (:`Triggered`
    (set `self.ControleDeCamera?` true)
    (`SceneComponent.K2_SetRelativeRotation` (`self.SpringArm`) (`KismetMathLibrary.RInterpTo` (`SceneComponent.RelativeRotation` (`self.SpringArm`)) (`KismetMathLibrary.MakeRotator` 0.0 (`KismetMathLibrary.FClamp` (+ (* ActionValue_Y _sensibilitevue) _relativerotation_pitch) (`self.VueMinimum_Y`) (`self.VueMaximum_Y`)) (`KismetMathLibrary.FClamp` (+ (* ActionValue_X _sensibilitevue) _relativerotation_yaw) (`self.VueMinimum_X`) (`self.VueMaximum_X`))) (`GameplayStatics.GetWorldDeltaSeconds`) 15.0) false false))
  (:`Canceled`
    (`KismetSystemLibrary.Delay` (`self.DelaiRepositionnementCamera`) :!label _label_2)
    (set `self.ControleDeCamera?` false))
  (:`Completed`
    (goto _label_2)))

(event `EnhancedInput|/Game/Controls/Inputs/IA_ChangementVue`
  (params (ActionValue :type Boolean) (ElapsedSeconds :type "Float (double-precision)") (TriggeredSeconds :type "Float (double-precision)") (InputAction :type "InputAction Object Reference" :default "/Game/Controls/Inputs/IA_ChangementVue.IA_ChangementVue"))
  (bind _springarm (`self.SpringArm`))
  (bind _springarm_2 (`self.SpringArm`))
  ;[1 1 1] Controle de la caméra avec souris et manette
  ;;[1 1 1] Changement de vue, de la première personne à la troisième personne et vice-versa
  (:`Started`
    (`/Engine/EditorBlueprintResources/StandardMacros.FlipFlop`
      (:`A`
        ;;;[1 1 1] Paramètres de la vue à la première personne
        (set `SpringArmComponent.TargetArmLength` 0.0 _springarm)
        (set `SpringArmComponent.TargetOffset` (0.0 0.0 250.0) _springarm)
        (set `self.VueMinimum_Y` -25.0)
        (set `self.VueMaximum_Y` 35.0)
        (set `self.VueMinimum_X` -50.0)
        (set `self.VueMaximum_X` 40.0))
      (:`B`
        ;;;[1 1 1] Paramètres de la vue à la troisième personne
        (set `SpringArmComponent.TargetArmLength` 1500.0 _springarm_2)
        (set `SpringArmComponent.TargetOffset` (0.0 0.0 500.0) _springarm_2)
        (set `self.VueMinimum_Y` -360.0)
        (set `self.VueMaximum_Y` 360.0)
        (set `self.VueMinimum_X` -360.0)
        (set `self.VueMaximum_X` 360.0)))))

(event `Avancer_IA`
  (bind _velocitelocale_x (`KismetMathLibrary.BreakVector` (`self.VelociteLocale`)))
  (bind _datatablebateau_infos_vitessebateau (break `/Game/Blueprint/Bateaux/Bobbie/Struct_Boats` (`self.DataTableBateau_Infos`)))
  (bind _datatablebateau_infos_vitessebateau_2 (break `/Game/Blueprint/Bateaux/Bobbie/Struct_Boats` (`self.DataTableBateau_Infos`)))
  ;[1 1 1] Controôle des mouvements
  ;;[1 1 1] Input pour accélérer
  (set `self.Acceleration_IA` true)
  ;;;[1 1 1] Limiteur de vitesse
  (if (<= (`self.VelociteGlobale`) (/ _datatablebateau_infos_vitessebateau 2.0)) :!label _label_3
    (if (`self.Acceleration_IA`)
      ;;;[1 1 1] S'assure d'être dans l'eau pour pouvoir avancer
      (if (`BuoyancyComponent.IsInWaterBody` (`self.Buoyancy1`)) :!label _label_4
        (`PrimitiveComponent.AddForceAtLocationLocal` (`self.SM_Bobbie`) (`KismetMathLibrary.MakeVector` (* (`KismetMathLibrary.SelectFloat` 1.0 (stale `EnhancedInput|/Game/Controls/Inputs/IA_Throttle` ActionValue) (`self.Acceleration_IA`)) (* (`KismetMathLibrary.FClamp` (`KismetMathLibrary.SelectFloat` 5.0 (stale `EnhancedInput|/Game/Controls/Inputs/IA_Throttle` TriggeredSeconds) (`self.Acceleration_IA`)) (`KismetMathLibrary.SelectFloat` 1.0 10.0 (> _velocitelocale_x 700.0)) 5.0) _datatablebateau_infos_vitessebateau_2))) (0.0 0.0 0.0) "None"))
      (elif (> (stale `EnhancedInput|/Game/Controls/Inputs/IA_Throttle` ActionValue) 0.0)
        (goto _label_4)))))

(event `EnhancedInput|/Game/Controls/Inputs/IA_Throttle`
  (params (ActionValue :type "Float (double-precision)") (ElapsedSeconds :type "Float (double-precision)") (TriggeredSeconds :type "Float (double-precision)") (InputAction :type "InputAction Object Reference" :default "/Game/Controls/Inputs/IA_Throttle.IA_Throttle"))
  ;[1 1 1] Controôle des mouvements
  ;;[1 1 1] Input pour accélérer
  (:`Triggered`
    (set `self.Acceleration_IA` false)
    (goto _label_3)))

(event `EnhancedInput|/Game/Controls/Inputs/IA_SteerLeft`
  (params (ActionValue :type "Float (double-precision)") (ElapsedSeconds :type "Float (double-precision)") (TriggeredSeconds :type "Float (double-precision)") (InputAction :type "InputAction Object Reference" :default "/Game/Controls/Inputs/IA_SteerLeft.IA_SteerLeft"))
  (bind (_datatablebateau_infos_vitessebateau _datatablebateau_infos_forcededirection) (break `/Game/Blueprint/Bateaux/Bobbie/Struct_Boats` (`self.DataTableBateau_Infos`)))
  (bind _returnvalue (* (`KismetMathLibrary.FClamp` TriggeredSeconds 0.5 3.0) (* (* ActionValue _datatablebateau_infos_forcededirection) -1.0)))
  ;[1 1 1] Controôle des mouvements
  ;;[1 1 1] Rotation vers la gauche à l'appui du input correspndant.
  (:`Triggered`
    (if (`BuoyancyComponent.IsInWaterBody` (`self.Buoyancy1`))
      (`PrimitiveComponent.AddForceAtLocationLocal` (`self.SM_Bobbie`) (`KismetMathLibrary.MakeVector` 0.0 _returnvalue) (300.0 250.0 100.0) "None")
      ;;;[1 1 1] Force arrière Droite pour assister la rotation de gauche
      (`PrimitiveComponent.AddForceAtLocationLocal` (`self.SM_Bobbie`) (`KismetMathLibrary.MakeVector` 0.0 (/ (* _returnvalue -1.0) 2.0)) (-300.0 -150.0 100.0) "None"))))

(event `EnhancedInput|/Game/Controls/Inputs/IA_SteerRight`
  (params (ActionValue :type "Float (double-precision)") (ElapsedSeconds :type "Float (double-precision)") (TriggeredSeconds :type "Float (double-precision)") (InputAction :type "InputAction Object Reference" :default "/Game/Controls/Inputs/IA_SteerRight.IA_SteerRight"))
  (bind (_datatablebateau_infos_vitessebateau _datatablebateau_infos_forcededirection) (break `/Game/Blueprint/Bateaux/Bobbie/Struct_Boats` (`self.DataTableBateau_Infos`)))
  (bind _returnvalue (* (`KismetMathLibrary.FClamp` TriggeredSeconds 0.5 3.0) (* ActionValue _datatablebateau_infos_forcededirection)))
  ;[1 1 1] Controôle des mouvements
  ;;[1 1 1] Rotation vers la droite à l'appui du input correspndant.
  (:`Triggered`
    (if (`BuoyancyComponent.IsInWaterBody` (`self.Buoyancy1`))
      (`PrimitiveComponent.AddForceAtLocationLocal` (`self.SM_Bobbie`) (`KismetMathLibrary.MakeVector` 0.0 _returnvalue) (300.0 -250.0 100.0) "None")
      ;;;[1 1 1] Force arrière Gauche pour assister la rotation de `Droit
      (`PrimitiveComponent.AddForceAtLocationLocal` (`self.SM_Bobbie`) (`KismetMathLibrary.MakeVector` 0.0 (/ (* _returnvalue -1.0) 2.0)) (-300.0 150.0 100.0) "None"))))

(event `Freinage_AI`
  (bind (_datatablebateau_infos_vitessebateau _datatablebateau_infos_forcededirection _datatablebateau_infos_forcedefreinage) (break `/Game/Blueprint/Bateaux/Bobbie/Struct_Boats` (`self.DataTableBateau_Infos`)))
  (bind (_datatablebateau_infos_vitessebateau_2 _datatablebateau_infos_forcededirection_2 _datatablebateau_infos_forcedefreinage_2) (break `/Game/Blueprint/Bateaux/Bobbie/Struct_Boats` (`self.DataTableBateau_Infos`)))
  (bind _velociteglobale (`self.VelociteGlobale`))
  (bind (_datatablebateau_infos_vitessebateau_3 _datatablebateau_infos_forcededirection_3 _datatablebateau_infos_forcedefreinage_3) (break `/Game/Blueprint/Bateaux/Bobbie/Struct_Boats` (`self.DataTableBateau_Infos`)))
  (bind (_returnvalue_x _returnvalue_y) (`KismetMathLibrary.BreakVector` (`KismetMathLibrary.Normal` (`self.VelociteLocale`))))
  (bind _returnvalue (> _velociteglobale 700.0))
  ;[1 1 1] Controôle des mouvements
  ;;[1 1 1] Pour le controle au clavier seulement
  (set `self.Freinage_IA` true)
  (if (and (< (stale `EnhancedInput|/Game/Controls/Inputs/IA_Reverse` ActionValue) 0.0) (< _velociteglobale _datatablebateau_infos_forcedefreinage_3) (not (`self.Freinage_IA`))) :!label _label_5
    ;;;[1 1 1] S'assure que le bateau est dans l'eau
    (if (`BuoyancyComponent.IsInWaterBody` (`self.Buoyancy1`)) :!label _label_6
      (bind _returnvalue_2 (* (`KismetMathLibrary.FClamp` (stale `EnhancedInput|/Game/Controls/Inputs/IA_Reverse` TriggeredSeconds) (`KismetMathLibrary.SelectFloat` 5.0 10.0 _returnvalue) 10.0) _datatablebateau_infos_forcedefreinage))
      (`PrimitiveComponent.AddForceAtLocationLocal` (`self.SM_Bobbie`) (`KismetMathLibrary.SelectVector` (* (* _returnvalue_2 (`KismetMathLibrary.MakeVector` _returnvalue_x _returnvalue_y)) -1.0) (`KismetMathLibrary.MakeVector` (* _returnvalue_2 -1.0)) _returnvalue) (0.0 0.0 0.0) "None"))
    (elif (and (`self.Freinage_IA`) (< (`self.VelociteGlobale`) _datatablebateau_infos_forcedefreinage_2))
      (goto _label_6))))

(event `EnhancedInput|/Game/Controls/Inputs/IA_Reverse`
  (params (ActionValue :type "Float (double-precision)") (ElapsedSeconds :type "Float (double-precision)") (TriggeredSeconds :type "Float (double-precision)") (InputAction :type "InputAction Object Reference" :default "/Game/Controls/Inputs/IA_Reverse.IA_Reverse"))
  ;[1 1 1] Controôle des mouvements
  ;;[1 1 1] Pour le controle au clavier seulement
  (:`Triggered`
    (goto _label_5)))

(event `self.SM_Bobbie.OnComponentHit`
  (params (HitComponent :type "PrimitiveComponent Object Reference") (OtherActor :type "Actor Object Reference") (OtherComp :type "PrimitiveComponent Object Reference") (NormalImpulse :type "Vector Structure") (Hit :type "HitResult Structure (by ref)"))
  (bind _dommagerecu (`self.DommageRecu`))
  (bind _returnvalue (`KismetMathLibrary.VSize` (`self.GetVelocity`)))
  ;[1 1 1] Comportement lors d'un impacte avec un obstacle de l'environnement
  ;;[1 1 1] Vérifie si le joueur est immunisé contre la collision actuelle.
  (if (not (`self.Collision?`))
    (set `self.Collision?` true)
    ;;[1 1 1] Évalue la vitesse de Bobbie pour appliquer les dommages respectif.
    (`self.ForceFeedbackSetup` "/Game/Controls/Feedback/FF_Collision.FF_Collision" false 1.0)
    (if (> _returnvalue 500.0)
      (if (> _returnvalue 1500.0)
        ;;[1 1 1] Enlève plus de vie à Bobbie vu l'impacte plus fort. Autant dans le Blueprint que dans le UI
        (bind (_vierestante _mort_) (`self.Retrait de Vie` (* _dommagerecu 2.0)))
        (if (not _mort_)
          ;;[1 1 1] Offre une invicibilité temporaire entre les collision (Temps configurable)
          (`KismetSystemLibrary.Delay` (`self.TempsImmunite`))
          (set `self.Collision?` false))
        (else
          ;;[1 1 1] Enlève de la vie à Bobbie. Autant dans le Blueprint que dans le UI
          (bind (_vierestante_2 _mort__2) (`self.Retrait de Vie` _dommagerecu))
          (if (not _mort__2)
            ;;[1 1 1] Offre une invicibilité temporaire entre les collision (Temps configurable)
            (`KismetSystemLibrary.Delay` (`self.TempsImmunite`))
            (set `self.Collision?` false))))
      (else
        (`KismetSystemLibrary.Delay` (`self.TempsImmunite`))
        (set `self.Collision?` false)))))

(event `InitialisationFocusForce`
  (params (Selection :type "/Game/Blueprint/Bateaux/Bobbie/Enum_LookAtTargets Enum" :default "NewEnumerator0"))
  ;[1 0.6024 0.2067] Controle de la rotation lors d'un focus forcé de la camera sur un objet
  ;;[1 1 1] hCustene
  (bind _output_get (set `self.SujetFocus` Selection))
  (`self.DisableInput` (`GameplayStatics.GetPlayerController` 0))
  (switch `/Game/Blueprint/Bateaux/Bobbie/Enum_LookAtTargets` _output_get
    (:`NewEnumerator0`
      (bind _returnvalue (`GameplayStatics.GetActorOfClass` "/Game/Blueprint/Naufrages/BP_FuseeDetresse.BP_FuseeDetresse_C"))
      (`/Engine/EditorBlueprintResources/StandardMacros.IsValid` _returnvalue
        (:`Is Valid`
          (set `self.CibleFocus` _returnvalue)
          (set `self.RegardForce` true))))))

(event `FocusNaufrage`
  ;[1 0.6024 0.2067] Controle de la rotation lors d'un focus forcé de la camera sur un objet
)

(fn `CalculContreForceLateral`
  (returns (`Contre Force` :type "Float (double-precision)") (`Glissement?` :type Boolean))
  (bind (_velocitelocale_x _velocitelocale_y) (`KismetMathLibrary.BreakVector` (`self.VelociteLocale`)))
  (bind _returnvalue (- _velocitelocale_x _velocitelocale_y))
  (`self.Print_Infos` "ForceLaterale" (`KismetStringLibrary.Conv_DoubleToString` _velocitelocale_y) (struct :`R` 1.0 :`G` 0.867631 :`A` 1.0))
  (`self.Print_Infos` "Transfert De force" (`KismetStringLibrary.Conv_DoubleToString` _returnvalue) (struct :`R` 1.0 :`G` 0.521295 :`A` 1.0))
  (return _returnvalue (or (> _velocitelocale_y 100.0) (< _velocitelocale_y -100.0))))

(fn `ForceFeedbackSetup`
  (params (`Effet Force Feedback` :type "ForceFeedbackEffect Object Reference") (Looping :type Boolean) (`Intensite Force Feeback` :type "Float (single-precision)"))
  (bind _forcefeedback (`self.ForceFeedback`))
  (`ForceFeedbackComponent.SetForceFeedbackEffect` _forcefeedback `Effet Force Feedback`)
  (set `ForceFeedbackComponent.bLooping` Looping _forcefeedback)
  (`ForceFeedbackComponent.SetIntensityMultiplier` _forcefeedback `Intensite Force Feeback`))

(fn `Print_Infos`
  (params (`Nom de la valeur` :type String) (Valeur :type String) (`Couleur du texte` :type "LinearColor Structure") (Duration :type "Float (single-precision)") (bPrintToScreen :type Boolean :default true))
  (`KismetSystemLibrary.PrintString` (`KismetStringLibrary.Concat_StrStr` `Nom de la valeur` Valeur) bPrintToScreen true `Couleur du texte` Duration))

(fn `Retrait de Vie`
  (params (`Vie retire` :type "Float (double-precision)"))
  (returns (VieRestante :type "Float (double-precision)") (`Mort?` :type Boolean))
  ;[1 1 1] Retire la vie dans le Blueprint pour ensuite mettre la variable à jour pour le widget
  (bind _output_get (set `self.SanteBobbie` (- (`self.SanteBobbie`) `Vie retire`)))
  (if (<= _output_get 0.0)
    (bind _output_get_2 (set `self.Mort?` true))
    (return 0.0 _output_get_2)
    (else
      (set `self.Mort?` false)
      ;[1 1 1] Met à jour la vie dans le UI du joueur
      (`/Game/Widget/WBP_UI_Jeu.EnleverVie` (`self.UI_EnJeu`))
      (return _output_get false))))

(fn `UserConstructionScript`
  (bind _springarm (`self.SpringArm`))
  (bind _datatable_ref (`self.DataTable_Ref`))
  (`|ExecutionSequence`
    (:`then_0`
      ;[1 1 1] Assignation au bon type de bateau
      (switch `/Game/Blueprint/Bateaux/Bobbie/Enum_TypeBateaux` (`self.TypeDeBatea`)
        (:`NewEnumerator4`
          (set `self.IndexBateau` 0))
        (:`NewEnumerator0`
          (set `self.IndexBateau` 1))
        (:`NewEnumerator1`
          (set `self.IndexBateau` 2))
        (:`NewEnumerator2`
          (set `self.IndexBateau` 3)))
      (`StaticMeshComponent.SetStaticMesh` (`self.SM_Bobbie`) (`|GetArrayItem` (`self.MeshesBateaux`) (`self.IndexBateau`)))
      (bind _outrownames (`DataTableFunctionLibrary.GetDataTableRowNames` _datatable_ref))
      (bind _returnvalue (`|GetDataTableRow` _datatable_ref (`|GetArrayItem` _outrownames (`self.IndexBateau`)))
        (:`then`
          (set `self.DataTableBateau_Infos` _returnvalue))))
    (:`then_1`
      ;[1 1 1] Positionnement de la caméra à la troisième personne
      (set `self.VueMinimum_Y` -360.0)
      (set `self.VueMaximum_Y` 360.0)
      (set `self.VueMinimum_X` -360.0)
      (set `self.VueMaximum_X` 360.0)
      (set `SpringArmComponent.TargetArmLength` 1500.0 _springarm)
      (set `SpringArmComponent.TargetOffset` (0.0 0.0 500.0) _springarm))))