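; Third-person player boat template whose construction script picks a mesh and data table stats (speed, steering force) from the chosen boat type.
; Throttle, reverse and steering apply local forces at offset points on the hull, scaled by hold time and only while buoyancy reports water.
; Tick applies velocity-based lateral counter-force against sliding and widens the camera FOV with speed.
; Mouse and gamepad look rotate the spring arm.
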(event `self.ReceiveBeginPlay`)

(event `self.ReceiveTick`
  (params (DeltaSeconds :type "Float (single-precision)"))
  (bind (_velocitelocale_x _velocitelocale_y) (`KismetMathLibrary.BreakVector` (`self.VelociteLocale`)))
  ;[1 1 1] Gestion  de la contre force appliqué sur le bateau lorsque l'on tourne.
  (set `self.VelociteLocale` (`KismetMathLibrary.InverseTransformDirection` (`self.GetTransform`) (`self.GetVelocity`)))
  (`|ExecutionSequence`
    (:`then_0`
      (`self.AjustementFieldOfView`))
    (:`then_1`
      (bind _contre_force (`self.GlissementLateralCheck`))
      (`PrimitiveComponent.AddForceAtLocationLocal` (`self.SM_Bobbie`) (`KismetMathLibrary.MakeVector` (* _velocitelocale_x 1.0) (* _velocitelocale_y -50.0)) (0.0 0.0 0.0) "None")
      (`self.Print_Infos` "Force de poussé" (`KismetStringLibrary.Conv_DoubleToString` _contre_force) (struct :`G` 1.0 :`B` 0.364774 :`A` 1.0)))))

(event `EnhancedInput|/Game/Controls/Inputs/IA_LookAroundController`
  (params (ActionValue :type "Vector2D Structure") (ElapsedSeconds :type "Float (double-precision)") (TriggeredSeconds :type "Float (double-precision)") (InputAction :type "InputAction Object Reference" :default "/Game/Controls/Inputs/IA_LookAroundController.IA_LookAroundController"))
  (bind _sensibilitevue (`self.SensibiliteVue`))
  (bind (_relativerotation_roll _relativerotation_pitch _relativerotation_yaw) (`KismetMathLibrary.BreakRotator` (`SceneComponent.RelativeRotation` (`self.SpringArm`))))
  ;[1 1 1] Controle de la caméra avec souris et manette
  ;;[1 1 1] Mouvements et limitations de la caméra à la manette
  (:`Triggered`
    (bind _result (`/Engine/EditorBlueprintResources/StandardMacros.NegateFloat` (* ActionValue_Y _sensibilitevue))
      (:`  `
        (`SceneComponent.K2_SetRelativeRotation` (`self.SpringArm`) (`KismetMathLibrary.MakeRotator` 0.0 (`KismetMathLibrary.FClamp` (+ _result _relativerotation_pitch) -360.0 360.0) (`KismetMathLibrary.FClamp` (+ (* ActionValue_X _sensibilitevue) _relativerotation_yaw) -360.0 360.0)) false false)))))

(event `AjustementFieldOfView`
  (bind _velocitelocale_x (`KismetMathLibrary.BreakVector` (`self.VelociteLocale`)))
  ;[1 1 1] Controle de la caméra avec souris et manette
  ;;[1 1 1] Ajuste le field of view en fonction de la vitesse du bateau pour donner une impression de vitesse
  (`CameraComponent.SetFieldOfView` (`self.Camera`) (`KismetMathLibrary.MapRangeClamped` _velocitelocale_x 0.0 2000.0 (`self.FOVMinimum`) (`self.FOVMaximum`))))

(event `EnhancedInput|/Game/Controls/Inputs/IA_LookAroundMouse`
  (params (ActionValue :type "Vector2D Structure") (ElapsedSeconds :type "Float (double-precision)") (TriggeredSeconds :type "Float (double-precision)") (InputAction :type "InputAction Object Reference" :default "/Game/Controls/Inputs/IA_LookAroundMouse.IA_LookAroundMouse"))
  (bind _sensibilitevue (`self.SensibiliteVue`))
  (bind (_relativerotation_roll _relativerotation_pitch _relativerotation_yaw) (`KismetMathLibrary.BreakRotator` (`SceneComponent.RelativeRotation` (`self.SpringArm`))))
  ;[1 1 1] Controle de la caméra avec souris et manette
  ;;[1 1 1] Mouvements et limitations de la caméra à la souris
  (:`Triggered`
    (`SceneComponent.K2_SetRelativeRotation` (`self.SpringArm`) (`KismetMathLibrary.MakeRotator` 0.0 (`KismetMathLibrary.FClamp` (+ (* ActionValue_Y _sensibilitevue) _relativerotation_pitch) -360.0 360.0) (`KismetMathLibrary.FClamp` (+ (* ActionValue_X _sensibilitevue) _relativerotation_yaw) -360.0 360.0)) false false)))

(event `EnhancedInput|/Game/Controls/Inputs/IA_Throttle`
  (params (ActionValue :type "Float (double-precision)") (ElapsedSeconds :type "Float (double-precision)") (TriggeredSeconds :type "Float (double-precision)") (InputAction :type "InputAction Object Reference" :default "/Game/Controls/Inputs/IA_Throttle.IA_Throttle"))
  (bind _datatablebateau_infos_vitessebateau (break `/Game/Blueprint/Bateaux/Struct_Boats` (`self.DataTableBateau_Infos`)))
  ;[1 1 1] Input pour accélérer
  (:`Triggered`
    ;;[1 1 1] S'assure d'être dans l'eau pour pouvoir avancer
    (if (`BuoyancyComponent.IsInWaterBody` (`self.Buoyancy`))
      (`PrimitiveComponent.AddForceAtLocationLocal` (`self.SM_Bobbie`) (`KismetMathLibrary.MakeVector` (* ActionValue (* (`KismetMathLibrary.FClamp` TriggeredSeconds 0.0 3.0) _datatablebateau_infos_vitessebateau))) (`KismetMathLibrary.MakeVector` (`KismetMathLibrary.FClamp` (* ActionValue -300.0) -150.0 -300.0)) "None"))))

(event `EnhancedInput|/Game/Controls/Inputs/IA_SteerLeft`
  (params (ActionValue :type Boolean) (ElapsedSeconds :type "Float (double-precision)") (TriggeredSeconds :type "Float (double-precision)") (InputAction :type "InputAction Object Reference" :default "/Game/Controls/Inputs/IA_SteerLeft.IA_SteerLeft"))
  (bind (_datatablebateau_infos_vitessebateau _datatablebateau_infos_forcededirection) (break `/Game/Blueprint/Bateaux/Struct_Boats` (`self.DataTableBateau_Infos`)))
  (bind _returnvalue (* (`KismetMathLibrary.FClamp` TriggeredSeconds 0.5 3.0) (* _datatablebateau_infos_forcededirection -1.0)))
  ;[1 1 1] Rotation vers la gauche à l'appui du input correspndant.
  (:`Triggered`
    (if (`BuoyancyComponent.IsInWaterBody` (`self.Buoyancy`))
      (`PrimitiveComponent.AddForceAtLocationLocal` (`self.SM_Bobbie`) (`KismetMathLibrary.MakeVector` 0.0 _returnvalue) (100.0 -250.0 0.0) "None")
      (`PrimitiveComponent.AddForceAtLocationLocal` (`self.SM_Bobbie`) (`KismetMathLibrary.MakeVector` 2500.0 (/ _returnvalue 2.0)) (-100.0 250.0 100.0) "None"))))

(event `EnhancedInput|/Game/Controls/Inputs/IA_SteerRight`
  (params (ActionValue :type Boolean) (ElapsedSeconds :type "Float (double-precision)") (TriggeredSeconds :type "Float (double-precision)") (InputAction :type "InputAction Object Reference" :default "/Game/Controls/Inputs/IA_SteerRight.IA_SteerRight"))
  (bind (_datatablebateau_infos_vitessebateau _datatablebateau_infos_forcededirection) (break `/Game/Blueprint/Bateaux/Struct_Boats` (`self.DataTableBateau_Infos`)))
  (bind _returnvalue (* (`KismetMathLibrary.FClamp` TriggeredSeconds 0.5 3.0) _datatablebateau_infos_forcededirection))
  ;[1 1 1] Rotation vers la droite à l'appui du input correspndant.
  (:`Triggered`
    (if (`BuoyancyComponent.IsInWaterBody` (`self.Buoyancy`))
      (`PrimitiveComponent.AddForceAtLocationLocal` (`self.SM_Bobbie`) (`KismetMathLibrary.MakeVector` 0.0 _returnvalue) (100.0 250.0 100.0) "None")
      (`PrimitiveComponent.AddForceAtLocationLocal` (`self.SM_Bobbie`) (`KismetMathLibrary.MakeVector` 2500.0 (/ _returnvalue 2.0)) (-100.0 -250.0 100.0) "None"))))

(event `EnhancedInput|/Game/Controls/Inputs/IA_Reverse`
  (params (ActionValue :type Boolean) (ElapsedSeconds :type "Float (double-precision)") (TriggeredSeconds :type "Float (double-precision)") (InputAction :type "InputAction Object Reference" :default "/Game/Controls/Inputs/IA_Reverse.IA_Reverse"))
  (bind _datatablebateau_infos_vitessebateau (break `/Game/Blueprint/Bateaux/Struct_Boats` (`self.DataTableBateau_Infos`)))
  ;[1 1 1] Pour le controle au clavier seulement
  (:`Triggered`
    ;;[1 1 1] S'assure que le bateau est dans l'eau
    (if (`BuoyancyComponent.IsInWaterBody` (`self.Buoyancy`))
      (`PrimitiveComponent.AddForceAtLocationLocal` (`self.SM_Bobbie`) (`KismetMathLibrary.MakeVector` (* (* (`KismetMathLibrary.FClamp` TriggeredSeconds 0.0 2.0) (/ _datatablebateau_infos_vitessebateau 100.0)) -1.0)) (0.0 100.0 0.0) "None"))))

(fn `GlissementLateralCheck`
  (returns (`Contre Force` :type "Float (double-precision)") (`Glissement?` :type Boolean))
  (bind (_velocitelocale_x _velocitelocale_y) (`KismetMathLibrary.BreakVector` (`self.VelociteLocale`)))
  (bind _returnvalue (or (> _velocitelocale_y 500.0) (< _velocitelocale_y -500.0)))
  (if _returnvalue
    (return (- (`self.VelociteMax`) _velocitelocale_y) _returnvalue)))

(fn `Print_Infos`
  (params (`Nom de la valeur` :type String) (Valeur :type String) (`Couleur du texte` :type "LinearColor Structure") (Duration :type "Float (single-precision)"))
  (`KismetSystemLibrary.PrintString` (`KismetStringLibrary.Concat_StrStr` `Nom de la valeur` Valeur) true true `Couleur du texte` Duration))

(fn `UserConstructionScript`
  (bind _datatable_ref (`self.DataTable_Ref`))
  (switch `/Game/Blueprint/Bateaux/Enum_TypeBateaux` (`self.TypeDeBatea`)
    (:`NewEnumerator4`
      (set `self.IndexBateau` 0))
    (:`NewEnumerator0`
      (set `self.IndexBateau` 1))
    (:`NewEnumerator1`
      (set `self.IndexBateau` 2))
    (:`NewEnumerator2`
      (set `self.IndexBateau` 3)))
  (`StaticMeshComponent.SetStaticMesh` (`self.SM_Bobbie`) (`|GetArrayItem` (`self.MeshesBateaux`) (`self.IndexBateau`)))
  (bind _outrownames (`DataTableFunctionLibrary.GetDataTableRowNames` _datatable_ref))
  (bind _returnvalue (`|GetDataTableRow` _datatable_ref (`|GetArrayItem` _outrownames (`self.IndexBateau`)))
    (:`then`
      (set `self.DataTableBateau_Infos` _returnvalue))))