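; BP_BeefyDropActor is a physics-simulated dropped item in the BeefyBass VFX tools, with a configurable mesh and a food chain index.
; Construction applies the mesh, a random value and the initial struggle state, which drive the material through custom primitive data.
; The struggle animation is started by writing a wrapped game-time stamp.
; Query functions expose location, food chain index and a zero collision radius, while pickup destroys the actor.
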(event `self.ReceiveBeginPlay`
  (`PrimitiveComponent.SetSimulatePhysics` (`self.StaticMesh`) true))

(event `/Game/Vfx/BeefyBass/Blueprints/Interfaces/BPI_BeefyAnimation.SetRandomFloat`
  (params (`Random0-1` :type "Float (double-precision)"))
  (bind _output_get (set `self.Random 0-1` `Random0-1`))
  (`PrimitiveComponent.SetCustomPrimitiveDataFloat` (`self.StaticMesh`) 0 _output_get))

(event `/Game/Vfx/BeefyBass/Blueprints/Interfaces/BPI_BeefyAnimation.SetStrugglingAnimation`
  (params (Enable :type Boolean))
  (`PrimitiveComponent.SetCustomPrimitiveDataFloat` (`self.StaticMesh`) 1 (`KismetMathLibrary.SelectFloat` (mod (+ (`KismetSystemLibrary.GetGameTimeInSeconds`) -0.05) 100.0) -1.0 Enable))
  (`PrimitiveComponent.SetCustomPrimitiveDataFloat` (`self.StaticMesh`) 7 (`KismetMathLibrary.SelectFloat` -1.0 0.0 Enable)))

(event `/Game/Vfx/BeefyBass/Blueprints/Interfaces/BPI_BeefyAnimation.SetMesh`
  (params (Mesh :type "StaticMesh Object Reference"))
  (if (`KismetSystemLibrary.IsValid` Mesh)
    (`StaticMeshComponent.SetStaticMesh` (`self.StaticMesh`) Mesh)))

(event `/Game/Vfx/BeefyBass/Blueprints/Interfaces/BPI_BeefyAnimation.SetFoodChainIndex`
  (params (Index :type Integer))
  (set `self.FoodChainIndex` Index))

(fn `GetCollisionRadius`
  (returns (CollisionRadius :type "Float (double-precision)"))
  (return 0.0))

(fn `GetFoodChainIndex`
  (returns (Index :type Integer))
  (return (`self.FoodChainIndex`)))

(fn `GetLocationWorldSpace`
  (returns (Location :type "Vector Structure"))
  (return (`SceneComponent.K2_GetComponentLocation` (`self.StaticMesh`))))

(fn `PickupItem`
  (params (Location :type "Vector Structure") (Radius :type "Float (double-precision)") (CheckLocation :type Boolean))
  (returns (ItemClass :type "Actor Class Reference"))
  (`self.K2_DestroyActor`)
  (return "BP_BeefyDropActor_C"))

(fn `UserConstructionScript`
  (`self.SetRandomFloat` (`self.Random 0-1`))
  (`self.SetStrugglingAnimation` (`self.InitialStruggle`))
  (`self.SetMesh` (`self.Mesh`)))